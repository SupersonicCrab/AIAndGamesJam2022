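; Wave manager that runs timed enemy waves from a data table and reports a win to GM_DwarfStuck when they run out.
; StartWave spawns each row's enemies at random BP_EnemySpawners, plays its music track and sets a timer for NextWave.
; BeginPlay caches spawners, music manager, total wave length and wave count.
; It also tracks active enemies and resources, flagging resource availability on the collection robot's blackboard.
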(event `self.ReceiveBeginPlay`
  (`parent.ReceiveBeginPlay`)
  (bind (_totalwavelength _lastwaveindex) (`self.GetWaveInfo` (`self.WaveAsset`)))
  (set `self.TotalWaveLength` _totalwavelength)
  (set `self.LastWaveIndex` _lastwaveindex)
  (bind _outactors (`GameplayStatics.GetAllActorsOfClass` "/Game/NPCs/WaveManger/BP_EnemySpawner.BP_EnemySpawner_C"))
  (set `self.EnemySpawners` _outactors)
  (bind _returnvalue (`GameplayStatics.GetActorOfClass` "/Game/Blueprints/BP_MusicManager.BP_MusicManager_C"))
  (set `self.MusicManager` _returnvalue))

(fn `AddActiveEnemy`
  (params (Enemy :type "/Game/NPCs/Enemies/BP_EnemyCharacter Object Reference"))
  (`KismetArrayLibrary.Array_Add` (`self.ActiveEnemies`) Enemy))

(fn `AddActiveResource`
  (params (Resource :type "/Game/Blueprints/Resources/BP_Resource Object Reference (by ref)"))
  (`KismetArrayLibrary.Array_Add` (`self.ActiveResources`) Resource)
  (`self.UpdateCollectionRobotBlackboard`))

(fn `GetWaveInfo`
  (params (WaveTable :type "DataTable Object Reference"))
  (returns (TotalWaveLength :type "Float (double-precision)") (LastWaveIndex :type Integer))
  (locals (DataTableEntries :type "Array of Name") (Length :type "Float (double-precision)"))
  (bind _outrownames (`DataTableFunctionLibrary.GetDataTableRowNames` WaveTable))
  (bind _output_get (set `local.DataTableEntries` _outrownames))
  (for _array_element _output_get
    (bind _returnvalue (`|GetDataTableRow` (`self.WaveAsset`) _array_element)
      (:`then`
        (set `local.Length` (+ (`local.Length`) (`.WaveLength_4_8DE7275D4A937D688B85DBA09BE092AA` (break `/Game/NPCs/WaveManger/Waves/F_Wave` _returnvalue)))))))
  (return (`local.Length`) (`KismetArrayLibrary.Array_Length` _output_get)))

(fn `NextWave`
  (bind _currentwaveindex (`self.CurrentWaveIndex`))
  (bind _result (`/Engine/EditorBlueprintResources/StandardMacros.IncrementInt` _currentwaveindex)
    (:`  `
      (if (> _result (`self.LastWaveIndex`))
        (bind _asgm_dwarf_stuck (cast `/Game/Blueprints/GM_DwarfStuck` (`GameplayStatics.GetGameMode`)))
        (`/Game/Blueprints/GM_DwarfStuck.OnGameWon` _asgm_dwarf_stuck)
        (else
          (`self.StartWave` _currentwaveindex))))))

(fn `RemoveActiveEnemy`
  (params (Enemy :type "/Game/NPCs/Enemies/BP_EnemyCharacter Object Reference"))
  (`KismetArrayLibrary.Array_RemoveItem` (`self.ActiveEnemies`) Enemy))

(fn `RemoveActiveResource`
  (params (Resource :type "/Game/Blueprints/Resources/BP_Resource Object Reference (by ref)"))
  (`KismetArrayLibrary.Array_RemoveItem` (`self.ActiveResources`) Resource)
  (`self.UpdateCollectionRobotBlackboard`))

(fn `SpawnEnemies`
  (params (EnemiesToSpawn :type "Array of /Game/NPCs/WaveManger/Waves/F_EnemyToSpawn Structure"))
  (for _array_element EnemiesToSpawn
    (bind (_spawnclass _amounttospawn) (break `/Game/NPCs/WaveManger/Waves/F_EnemyToSpawn` _array_element))
    (if (> _amounttospawn 0)
      (for _ (range 1 (+ _amounttospawn 1))
        (`/Game/Blueprints/BP_CharacterSpawner.SpawnCharacterByClass` (`KismetArrayLibrary.Array_Random` (`self.EnemySpawners`)) _spawnclass)))))

(fn `StartWave`
  (params (WaveIndex :type Integer))
  (set `self.CurrentWaveIndex` WaveIndex)
  (bind _returnvalue (`|GetDataTableRow` (`self.WaveAsset`) (`KismetStringLibrary.Conv_StringToName` (`KismetStringLibrary.Conv_IntToString` WaveIndex)))
    (:`then`
      (bind (_enemiestospawn _wavelength _musictrack) (break `/Game/NPCs/WaveManger/Waves/F_Wave` _returnvalue))
      (`self.SpawnEnemies` _enemiestospawn)
      (`KismetSystemLibrary.K2_SetTimer` null "NextWave" _wavelength)
      (`/Game/Blueprints/BP_MusicManager.PlayTrack` (`self.MusicManager`) _musictrack))
    (:`RowNotFound`
      (bind _asgm_dwarf_stuck (cast `/Game/Blueprints/GM_DwarfStuck` (`GameplayStatics.GetGameMode`)))
      (`/Game/Blueprints/GM_DwarfStuck.OnGameWon` _asgm_dwarf_stuck))))

(fn `UpdateCollectionRobotBlackboard`
  (`BlackboardComponent.SetValueAsBool` (`self.CollectionRobotBlackboard`) "bResourcesAvailable" (not (`KismetArrayLibrary.Array_IsEmpty` (`self.ActiveResources`)))))

(fn `UserConstructionScript`)