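; Collection robot NPC that gathers magic and metal resources and deposits them with the DwarfStuck game mode.
; CollectResource takes the blackboard's TargetResource, adds its yield to a carried total, plays a type-specific sound and notifies the resource it is destroyed.
; A held-pickup count drives the bFullInventory blackboard key.
; DepositResources passes non-empty totals to the game mode, clears inventory and flag, and plays a crafting sound.
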(event `self.ReceiveBeginPlay`
  (`parent.ReceiveBeginPlay`)
  (bind _asgm_dwarf_stuck (cast `/Game/Blueprints/GM_DwarfStuck` (`GameplayStatics.GetGameMode`)))
  (set `self.GameMode` _asgm_dwarf_stuck))

(fn `CollectResource`
  (bind (_collectedresources_magic _collectedresources_metal) (break `/Game/Blueprints/F_ResourceAmount` (`self.CollectedResources`)))
  (bind _asbp_resource (cast `/Game/Blueprints/Resources/BP_Resource` (`BlackboardComponent.GetValueAsObject` (`self.Blackboard`) "TargetResource")))
  (`|ExecutionSequence`
    (:`then_0`
      (bind (_resourcesgained_magic _resourcesgained_metal) (break `/Game/Blueprints/F_ResourceAmount` (`/Game/Blueprints/Resources/BP_Resource.ResourcesGained` _asbp_resource)))
      (set `self.CollectedResources` (make `/Game/Blueprints/F_ResourceAmount` (+ _collectedresources_magic _resourcesgained_magic) (+ _collectedresources_metal _resourcesgained_metal))))
    (:`then_1`
      (bind _result (`/Engine/EditorBlueprintResources/StandardMacros.IncrementInt` (`self.ResourcesHeld`))
        (:`  `
          (`BlackboardComponent.SetValueAsBool` (`self.Blackboard`) "bFullInventory" (> _result (`self.MaxHeld`))))))
    (:`then_2`
      (`GameplayStatics.PlaySoundAtLocation` (select `bool` (== (`GameplayStatics.GetObjectClass` _asbp_resource) "/Game/Blueprints/Resources/BP_Magic.BP_Magic_C") :`false` "/Game/Assets/Audio/Effects/A_MetalCollected.A_MetalCollected" :`true` "/Game/Assets/Audio/Effects/A_MDPPlaced.A_MDPPlaced" :!type "SoundBase Object Reference") (`self.K2_GetActorLocation`) (struct) 0.5 1.0 0.0 null null null null)
      (`/Game/Blueprints/Resources/BP_Resource.OnResourceDestroyed` _asbp_resource))))

(fn `DepositResources`
  (bind (_collectedresources_magic _collectedresources_metal) (break `/Game/Blueprints/F_ResourceAmount` (`self.CollectedResources`)))
  (if (or (> _collectedresources_magic 0) (> _collectedresources_metal 0))
    (`/Game/Blueprints/GM_DwarfStuck.AddResources` (`self.GameMode`) (`self.CollectedResources`))
    (set `self.CollectedResources` (struct))
    (`BlackboardComponent.SetValueAsBool` (`self.Blackboard`) "bFullInventory" false)
    (set `self.ResourcesHeld` 0)
    (`GameplayStatics.PlaySoundAtLocation` "/Game/Assets/Audio/Effects/A_Crafting.A_Crafting" (`self.K2_GetActorLocation`) (struct) 1.0 1.0 0.0 null null null null)))

(fn `UserConstructionScript`
  (`parent.UserConstructionScript`))