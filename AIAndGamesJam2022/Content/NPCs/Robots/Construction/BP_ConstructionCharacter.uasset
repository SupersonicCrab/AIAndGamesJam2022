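; Construction robot character that carries a placeable and sets it down on a grid.
; AttachPlaceable snaps a valid placeable to the attach spot and records it in the Blackboard for AI use.
; DetachPlaceable teleports it to the placement location from Grid, assigns it to that grid, fires OnPlaced, then clears both references.
; The event graph is inactive, and Grid is assigned outside these graphs.
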(fn `AttachPlaceable`
  (params (Placeable :type "/Game/Blueprints/Placeables/BP_Placeable Object Reference"))
  (locals (PlaceableName :type Name :default "Placeable"))
  (`/Engine/EditorBlueprintResources/StandardMacros.IsValid` Placeable
    (:`Is Valid`
      (bind _output_get (set `self.Placeable` Placeable))
      (`self.K2_AttachToComponent` _output_get (`self.PlaceableAttachSpot`) "None" "SnapToTarget" "SnapToTarget" "SnapToTarget" true)
      (`BlackboardComponent.SetValueAsObject` (`self.Blackboard`) (`local.PlaceableName`) (`self.Placeable`)))))

(fn `DetachPlaceable`
  (bind _placeable (`self.Placeable`))
  (`self.K2_DetachFromActor` _placeable "KeepRelative" "KeepRelative" "KeepRelative")
  (bind _impactpoint (`/Game/Blueprints/PlayArea/BP_Grid.GetPlacementLocation` (`self.Grid`)))
  (`self.K2_SetActorLocation` _placeable _impactpoint false true)
  (bind _output_get (set `/Game/Blueprints/PlayArea/BP_Grid.Placeable` (`self.Placeable`) (`self.Grid`)))
  (`/Game/Blueprints/Placeables/BP_Placeable.OnPlaced` _output_get)
  (set `self.Placeable` null)
  (set `self.Grid` null))

(fn `UserConstructionScript`
  (`parent.UserConstructionScript`))