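; Base enemy character that registers with the wave manager and drops resources when killed.
; On BeginPlay it copies the obstruction checker's gate-blocked state into its Blackboard and caches its default walk speed.
; Damage reduces Health and prints a debug message; at zero, OnDeath spawns a poof effect, scatters Magic and Metal pickups randomly within SpawnRange, deregisters from the wave manager and destroys the actor.
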(event `self.ReceiveBeginPlay`
  (`parent.ReceiveBeginPlay`)
  (`self.UpdateGateObstructed`)
  (set `self.DefaultWalkSpeed` (`CharacterMovementComponent.MaxWalkSpeed` (`self.CharacterMovement`)))
  (bind _returnvalue (`GameplayStatics.GetActorOfClass` "/Game/NPCs/WaveManger/BP_WaveManager.BP_WaveManager_C"))
  (set `self.WaveManager` _returnvalue)
  (`/Game/NPCs/WaveManger/BP_WaveManager.AddActiveEnemy` _returnvalue self))

(event `self.ReceiveAnyDamage`
  (params (Damage :type "Float (single-precision)") (DamageType :type "DamageType Object Reference") (InstigatedBy :type "Controller Object Reference") (DamageCauser :type "Actor Object Reference"))
  (bind _output_get (set `self.Health` (- (`self.Health`) Damage)))
  (bind _returnvalue (<= _output_get 0.0))
  (`KismetSystemLibrary.PrintString` (`KismetStringLibrary.Concat_StrStr` (`KismetSystemLibrary.GetObjectName` self) (`KismetMathLibrary.SelectString` " was killed by " " was damaged by " _returnvalue) (`KismetSystemLibrary.GetObjectName` DamageCauser) " doing " (`KismetStringLibrary.Conv_DoubleToString` Damage) " damage") true true (struct :`G` 0.66 :`B` 1.0 :`A` 1.0) 5.0)
  (if _returnvalue
    (`self.OnDeath` true)))

(fn `OnDeath`
  (params (bSpawnResources :type Boolean :default true))
  (bind (_returnvalue_x _returnvalue_y _returnvalue_z) (`KismetMathLibrary.BreakVector` (`self.K2_GetActorLocation`)))
  (`|ExecutionSequence`
    (:`then_0`
      (`|SpawnActorFromClass` "/Game/Blueprints/AnimatedSprites/BP_Poof.BP_Poof_C" (`KismetMathLibrary.MakeTransform` (`KismetMathLibrary.MakeVector` (- _returnvalue_x 100.0) _returnvalue_y (+ _returnvalue_z (`CapsuleComponent.GetScaledCapsuleHalfHeight` (`self.CapsuleComponent`))))) "Undefined" "OverrideRootScale" null null)
      (if bSpawnResources
        (`self.SpawnResources`)))
    (:`then_1`
      (`/Game/NPCs/WaveManger/BP_WaveManager.RemoveActiveEnemy` (`self.WaveManager`) self))
    (:`then_2`
      (`self.K2_DestroyActor`))))

(fn `SpawnResource`
  (params (ResourceClass :type "/Game/Blueprints/Resources/BP_Resource Class Reference"))
  (locals (SpawnRange :type "Vector Structure" :default (30.0 30.0 0.0)))
  (bind (_spawnrange_x _spawnrange_y _spawnrange_z) (`KismetMathLibrary.BreakVector` (`local.SpawnRange`)))
  (`|SpawnActorFromClass` ResourceClass (`KismetMathLibrary.MakeTransform` (+ (`self.K2_GetActorLocation`) (`KismetMathLibrary.MakeVector` (`KismetMathLibrary.RandomFloatInRange` (* _spawnrange_x -1.0) _spawnrange_x) (`KismetMathLibrary.RandomFloatInRange` (* _spawnrange_y -1.0) _spawnrange_y) (`KismetMathLibrary.RandomFloatInRange` (* _spawnrange_z -1.0) _spawnrange_z)))) "AdjustIfPossibleButAlwaysSpawn" "OverrideRootScale" null null))

(fn `SpawnResources`
  (bind (_resourcesdropped_magic _resourcesdropped_metal) (break `/Game/Blueprints/F_ResourceAmount` (`self.ResourcesDropped`)))
  (bind _resourcesdropped_magic_2 (break `/Game/Blueprints/F_ResourceAmount` (`self.ResourcesDropped`)))
  (`|ExecutionSequence`
    (:`then_0`
      (if (> _resourcesdropped_magic_2 0)
        (for _ (range 1 (+ _resourcesdropped_magic_2 1))
          (`self.SpawnResource` "/Game/Blueprints/Resources/BP_Magic.BP_Magic_C"))))
    (:`then_1`
      (if (> _resourcesdropped_metal 0)
        (for _ (range 1 (+ _resourcesdropped_metal 1))
          (`self.SpawnResource` "/Game/Blueprints/Resources/BP_Metal.BP_Metal_C"))))))

(fn `UpdateGateObstructed`
  (bind _returnvalue (`GameplayStatics.GetActorOfClass` "/Game/NPCs/BP_ObstructionChecker.BP_ObstructionChecker_C"))
  (if (`/Game/NPCs/BP_ObstructionChecker.GateObstructed` _returnvalue)
    (`BlackboardComponent.SetValueAsBool` (`self.Blackboard`) "bGateObstructed" true)))

(fn `UserConstructionScript`
  (`parent.UserConstructionScript`))