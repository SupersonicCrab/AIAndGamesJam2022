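; Gnome enemy character that tracks nearby placeables and reports the closest one to its Blackboard.
; NearbyCollision overlaps maintain the placeable list, and only a new entry triggers the closest search.
; That search compares against a stored distance that is never reset here, and removals leave the target unchanged.
; BeginPlay increments the Blackboard's ActiveGnomes count and OnDeath decrements it before calling the parent death logic.
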(event `self.NearbyCollision.OnComponentBeginOverlap`
  (params (OverlappedComponent :type "PrimitiveComponent Object Reference") (OtherActor :type "Actor Object Reference") (OtherComp :type "PrimitiveComponent Object Reference") (OtherBodyIndex :type Integer) (bFromSweep :type Boolean) (SweepResult :type "HitResult Structure (by ref)"))
  (bind _nearbyplaceables (`self.NearbyPlaceables`))
  (bind _asbp_placeable (cast `/Game/Blueprints/Placeables/BP_Placeable` OtherActor))
  (if (not (`KismetArrayLibrary.Array_Contains` _nearbyplaceables _asbp_placeable))
    (`KismetArrayLibrary.Array_Add` _nearbyplaceables _asbp_placeable)
    (`self.SetClosestPlaceable`)))

(event `self.NearbyCollision.OnComponentEndOverlap`
  (params (OverlappedComponent :type "PrimitiveComponent Object Reference") (OtherActor :type "Actor Object Reference") (OtherComp :type "PrimitiveComponent Object Reference") (OtherBodyIndex :type Integer))
  (bind _asbp_placeable (cast `/Game/Blueprints/Placeables/BP_Placeable` OtherActor))
  (`KismetArrayLibrary.Array_RemoveItem` (`self.NearbyPlaceables`) _asbp_placeable))

(event `self.ReceiveBeginPlay`
  (bind _blackboard (`self.Blackboard`))
  (`parent.ReceiveBeginPlay`)
  (`BlackboardComponent.SetValueAsInt` _blackboard "ActiveGnomes" (+ (`BlackboardComponent.GetValueAsInt` _blackboard "ActiveGnomes") 1)))

(fn `OnDeath`
  (params (bSpawnResources :type Boolean))
  (bind _blackboard (`self.Blackboard`))
  (`BlackboardComponent.SetValueAsInt` _blackboard "ActiveGnomes" (- (`BlackboardComponent.GetValueAsInt` _blackboard "ActiveGnomes") 1))
  (`parent.OnDeath` bSpawnResources))

(fn `SetClosestPlaceable`
  (locals (ClosestPlaceable :type "/Game/Blueprints/Placeables/BP_Placeable Object Reference") (ClosestDistance :type "Float (double-precision)" :default 9999999.0))
  (if (not (`self.IsActorBeingDestroyed`))
    (for _array_element (`self.NearbyPlaceables`)
      (bind _returnvalue (`self.GetDistanceTo` _array_element self))
      (if (< _returnvalue (`local.ClosestDistance`))
        (set `local.ClosestPlaceable` _array_element)
        (set `local.ClosestDistance` _returnvalue)))
    (`BlackboardComponent.SetValueAsObject` (`self.Blackboard`) "ClosestPlaceable" (`local.ClosestPlaceable`))))

(fn `UserConstructionScript`
  (`parent.UserConstructionScript`))