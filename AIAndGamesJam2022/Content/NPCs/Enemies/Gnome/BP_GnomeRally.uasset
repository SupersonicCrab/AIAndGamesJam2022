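; BP_GnomeRally is a rally point that merges nearby gnome enemies into a single BP_GnomeTank.
; A sphere trigger tracks overlapping BP_GnomeCharacters, and each arrival restarts a RallyTime timer that calls CreateGnomeTank.
; If enough gnomes are present when it fires, it locks, kills the required number, spawns the tank at its own transform and destroys itself.
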(event `self.Sphere.OnComponentBeginOverlap`
  (params (OverlappedComponent :type "PrimitiveComponent Object Reference") (OtherActor :type "Actor Object Reference") (OtherComp :type "PrimitiveComponent Object Reference") (OtherBodyIndex :type Integer) (bFromSweep :type Boolean) (SweepResult :type "HitResult Structure (by ref)"))
  (if (not (`self.bSpawnLocked`))
    (bind _asbp_gnome_character (cast `/Game/NPCs/Enemies/Gnome/BP_GnomeCharacter` OtherActor))
    (`KismetArrayLibrary.Array_Add` (`self.NearbyGnomes`) _asbp_gnome_character)
    (`KismetSystemLibrary.K2_SetTimer` null "CreateGnomeTank" (`self.RallyTime`))))

(event `self.Sphere.OnComponentEndOverlap`
  (params (OverlappedComponent :type "PrimitiveComponent Object Reference") (OtherActor :type "Actor Object Reference") (OtherComp :type "PrimitiveComponent Object Reference") (OtherBodyIndex :type Integer))
  (if (not (`self.bSpawnLocked`))
    (bind _asbp_gnome_character (cast `/Game/NPCs/Enemies/Gnome/BP_GnomeCharacter` OtherActor))
    (`KismetArrayLibrary.Array_RemoveItem` (`self.NearbyGnomes`) _asbp_gnome_character)))

(fn `CreateGnomeTank`
  (if (and (>= (`KismetArrayLibrary.Array_Length` (`self.NearbyGnomes`)) (`self.GnomesRequired`)) (not (`self.bSpawnLocked`)))
    (set `self.bSpawnLocked` true)
    (`PrimitiveComponent.SetCollisionEnabled` (`self.Sphere`) "NoCollision")
    (for _index (range (`self.GnomesRequired`))
      (`/Game/NPCs/Enemies/BP_EnemyCharacter.OnDeath` (`|GetArrayItem` (`self.NearbyGnomes`) _index) false))
    (`|SpawnActorFromClass` "/Game/NPCs/Enemies/GnomeTank/BP_GnomeTank.BP_GnomeTank_C" (`self.GetTransform`) "AdjustIfPossibleButAlwaysSpawn" "OverrideRootScale" null null)
    (`self.K2_DestroyActor`)))

(fn `UserConstructionScript`
  (`parent.UserConstructionScript`))