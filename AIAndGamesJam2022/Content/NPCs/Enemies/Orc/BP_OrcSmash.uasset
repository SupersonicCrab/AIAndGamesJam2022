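; Orc enemy smash attack that deals area damage in a sphere centered on its owner.
; Execute runs the parent logic, draws a one-second debug sphere at Range, then gathers overlapping actors across several object types.
; Each actor that passes ActorIsValidTarget takes Damage, with the owner as damage causer.
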(fn `Execute`
  (bind _returnvalue (`self.GetOwner`))
  (bind _range (`self.Range`))
  (bind _returnvalue_2 (`Actor.K2_GetActorLocation` _returnvalue))
  (`parent.Execute`)
  (`KismetSystemLibrary.DrawDebugSphere` _returnvalue_2 _range 12 (struct :`R` 1.0 :`G` 1.0 :`B` 1.0 :`A` 1.0) 1.0 1.0)
  (bind _outactors (`KismetSystemLibrary.SphereOverlapActors` _returnvalue_2 _range (`|MakeArray` "ObjectTypeQuery8" "ObjectTypeQuery1" "ObjectTypeQuery3" "ObjectTypeQuery2" :!type "EObjectTypeQuery Enum")))
  (for _array_element _outactors
    (bind _validtarget (`self.ActorIsValidTarget` _array_element))
    (if _validtarget
      (`GameplayStatics.ApplyDamage` _array_element (`self.Damage`) null _returnvalue))))