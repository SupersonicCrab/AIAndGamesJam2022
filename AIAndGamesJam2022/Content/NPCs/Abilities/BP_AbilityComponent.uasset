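; BP_AbilityComponent is a timed ability component for a BP_SpriteCharacter NPC, with a warmup phase followed by a cooldown.
; It caches the owning character on BeginPlay, and Start acts only when ReadyToActivate, setting the character's sprite to the ability name during warmup.
; Function-name timers chain the phases: Start schedules Execute, which resets the sprite and schedules Finished to re-arm the ability after cooldown.
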(event `self.ReceiveBeginPlay`
  (`parent.ReceiveBeginPlay`)
  (bind _asbp_sprite_character (cast `/Game/Blueprints/BP_SpriteCharacter` (`self.GetOwner`)))
  (set `self.OwningSpriteCharacter` _asbp_sprite_character))

(fn `Execute`
  (`KismetSystemLibrary.K2_SetTimer` null "Finished" (`self.CooldownDuration`))
  (`/Game/Blueprints/BP_SpriteCharacter.UpdateSprite` (`self.OwningSpriteCharacter`) ""))

(fn `Finished`
  (set `self.bReadyToActivate` true))

(fn `Start`
  (if (`self.bReadyToActivate`)
    (set `self.bReadyToActivate` false)
    (`KismetSystemLibrary.K2_SetTimer` null "Execute" (`self.WarmupDuration`))
    (`/Game/Blueprints/BP_SpriteCharacter.UpdateSprite` (`self.OwningSpriteCharacter`) (`self.AbilityName`))))