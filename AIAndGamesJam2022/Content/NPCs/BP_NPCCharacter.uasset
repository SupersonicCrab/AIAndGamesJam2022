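; BP_NPCCharacter is an NPC character Blueprint that reports falling state to its AI Blackboard.
; BeginPlay caches the Blackboard after the parent logic runs.
; On each movement mode change it calls the parent, then, if the Blackboard is valid, writes the Falling bool.
; That bool comes from converting the new custom mode to a movement mode and comparing it to Falling, rather than reading the new movement mode.
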(event `self.K2_OnMovementModeChanged`
  (params (PrevMovementMode :type "EMovementMode Enum" :default "MOVE_None") (NewMovementMode :type "EMovementMode Enum" :default "MOVE_None") (PrevCustomMode :type Byte) (NewCustomMode :type Byte))
  (`parent.K2_OnMovementModeChanged` PrevMovementMode NewMovementMode PrevCustomMode NewCustomMode)
  (bind _blackboard (`self.Blackboard`)
    (:`then`
      (`BlackboardComponent.SetValueAsBool` _blackboard (`self.Falling`) (`|EnumEquality` (cast `EMovementMode` NewCustomMode) "MOVE_Falling")))
    (:`else`)))

(event `self.ReceiveBeginPlay`
  (`parent.ReceiveBeginPlay`)
  (set `self.Blackboard` (`AIBlueprintHelperLibrary.GetBlackboard` null)))

(fn `UserConstructionScript`
  (`parent.UserConstructionScript`))