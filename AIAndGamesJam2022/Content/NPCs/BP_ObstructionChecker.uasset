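; BP_ObstructionChecker tests whether a gate route is obstructed by querying a navigation path from its root to a Destination point.
; ObstructionCheck runs a synchronous path query with the NavFilter_PlayArea filter and treats a partial path as obstructed.
; It writes the result to a Blackboard key and the GateObstructed variable, then prints a debug message.
; RequestCheck debounces checks by restarting a delayed timer on each call.
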(fn `ObstructionCheck`
  (bind _returnvalue (`NavigationSystemV1.FindPathToLocationSynchronously` (`SceneComponent.K2_GetComponentLocation` (`self.DefaultSceneRoot`)) (`SceneComponent.K2_GetComponentLocation` (`self.Destination`)) null "/Game/NPCs/Navigation/NavFilter_PlayArea.NavFilter_PlayArea_C"))
  (bind _returnvalue_2 (`NavigationPath.IsPartial` _returnvalue))
  (`BlackboardComponent.SetValueAsBool` (`self.Blackboard`) (`self.GateObstructedName`) _returnvalue_2)
  (set `self.GateObstructed` _returnvalue_2)
  (`KismetSystemLibrary.PrintString` (`KismetStringLibrary.Concat_StrStr` "Path " (`KismetMathLibrary.SelectString` "obstructed" "clear" _returnvalue_2))))

(fn `RequestCheck`
  (params (CheckDelay :type "Float (double-precision)" :default 1.0))
  (`KismetSystemLibrary.K2_ClearTimer` null "ObstructionCheck")
  (`KismetSystemLibrary.K2_SetTimer` null "ObstructionCheck" CheckDelay))

(fn `UserConstructionScript`)