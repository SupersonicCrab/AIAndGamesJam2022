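; BP_Resource is a resource actor that the wave manager tracks while it is active in the level.
; On BeginPlay it finds BP_WaveManager with GetActorOfClass, caches the reference and registers itself as an active resource.
; OnResourceDestroyed removes it from the manager's active resources and then destroys the actor.
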(event `self.ReceiveBeginPlay`
  (`parent.ReceiveBeginPlay`)
  (bind _returnvalue (`GameplayStatics.GetActorOfClass` "/Game/NPCs/WaveManger/BP_WaveManager.BP_WaveManager_C"))
  (bind _output_get (set `self.WaveManager` _returnvalue))
  (`/Game/NPCs/WaveManger/BP_WaveManager.AddActiveResource` _output_get self))

(fn `OnResourceDestroyed`
  (`/Game/NPCs/WaveManger/BP_WaveManager.RemoveActiveResource` (`self.WaveManager`) self)
  (`self.K2_DestroyActor`))

(fn `UserConstructionScript`
  (`parent.UserConstructionScript`))