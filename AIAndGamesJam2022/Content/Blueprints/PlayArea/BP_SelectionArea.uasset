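; BP_SelectionArea is a play-area actor that fills its Bounds box with a lattice of BP_Grid actors.
; GenerateGrid runs on construction and BeginPlay, destroying tracked cells before spawning new ones.
; It divides the box's X and Y size by GridSize and spawns GridSize-wide cells at interior steps, sharing one computed height.
; Spawned cells are appended to Grids, which DestroyGrids iterates but never clears.
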(event `self.ReceiveBeginPlay`
  (`parent.ReceiveBeginPlay`)
  (`self.GenerateGrid`))

(fn `DestroyGrids`
  (for _array_element (`self.Grids`)
    (`self.K2_DestroyActor` _array_element)))

(fn `GenerateGrid`
  (locals (XSize :type Integer) (YSize :type Integer) (Extent :type "Vector Structure"))
  (bind (_returnvalue_x _returnvalue_y _returnvalue_z) (`KismetMathLibrary.BreakVector` (`self.K2_GetActorLocation`)))
  (bind _gridsize (`self.GridSize`))
  (bind (_extent_x _extent_y _extent_z) (`KismetMathLibrary.BreakVector` (`local.Extent`)))
  (bind (_returnvalue_x_2 _returnvalue_y_2 _returnvalue_z_2) (`KismetMathLibrary.BreakVector` (`BoxComponent.GetScaledBoxExtent` (`self.Bounds`))))
  (bind _returnvalue (/ (`self.GridSize`) 2.0))
  (set `local.Extent` (`KismetMathLibrary.MakeVector` _returnvalue_x_2 _returnvalue_y_2 _returnvalue_z_2))
  (set `local.XSize` (`.ReturnValue` (`KismetMathLibrary.FMod` (* _returnvalue_x_2 2.0) (`self.GridSize`))))
  (set `local.YSize` (`.ReturnValue` (`KismetMathLibrary.FMod` (* _returnvalue_y_2 2.0) (`self.GridSize`))))
  (`self.DestroyGrids`)
  (for _index (range 1 (`local.XSize`))
    (for _index_2 (range 1 (`local.YSize`))
      (bind _returnvalue_2 (`|SpawnActorFromClass` "/Game/Blueprints/PlayArea/BP_Grid.BP_Grid_C" (`KismetMathLibrary.MakeTransform` (`KismetMathLibrary.TransformLocation` (`self.GetTransform`) (`KismetMathLibrary.MakeVector` (- (* _index _gridsize) _extent_x) (- (* _index_2 _gridsize) _extent_y) (- (+ _returnvalue_z 128.0) (* _extent_z 2.0))))) "Undefined" "OverrideRootScale" null (`KismetMathLibrary.MakeVector` _returnvalue _returnvalue 150.0) null))
      (`KismetArrayLibrary.Array_Add` (`self.Grids`) _returnvalue_2))))

(fn `UserConstructionScript`
  (`parent.UserConstructionScript`)
  (`self.GenerateGrid`))