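; BP_Grid is a play-area actor that acts as a hoverable placement spot.
; OnHoverStarted and OnHoverFinished show and hide its Box component as a highlight.
; GetPlacementLocation line-traces WorldStatic objects vertically from the PlacementLocation component by PlacementRaycastLength and returns the impact point, without checking whether anything was hit.
; It has no event or construction logic of its own.
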(fn `GetPlacementLocation`
  (returns (ImpactPoint :type "Vector Structure"))
  (bind _returnvalue (`SceneComponent.K2_GetComponentLocation` (`self.PlacementLocation`)))
  (bind _outhit (`KismetSystemLibrary.LineTraceSingleForObjects` _returnvalue (+ _returnvalue (`KismetMathLibrary.MakeVector` 0.0 0.0 (`self.PlacementRaycastLength`))) (`|MakeArray` "ObjectTypeQuery1" :!type "EObjectTypeQuery Enum")))
  (return (`.ImpactPoint` (`GameplayStatics.BreakHitResult` _outhit))))

(fn `OnHoverFinished`
  (`SceneComponent.SetHiddenInGame` (`self.Box`) true false))

(fn `OnHoverStarted`
  (`SceneComponent.SetHiddenInGame` (`self.Box`) false false))

(fn `UserConstructionScript`)