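; BP_GameMode is the game mode that holds a pool of Magic and Metal resources and a health value for the game.
; SpendResources deducts a cost only if HasEnoughResources approves both amounts, prints the spend, and returns whether it succeeded.
; DealDamage clamps health between zero and the class-default Health, calling the empty OnGameOver hook and returning true at zero.
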(fn `DealDamage`
  (params (Damage :type "Float (double-precision)"))
  (returns (bLost :type Boolean))
  (bind _output_get (set `self.Health` (`KismetMathLibrary.FClamp` (- (`self.Health`) Damage) 0.0 (`.Health` (defaults `/Game/Blueprints/BP_GameMode` "BP_GameMode_C")))))
  (if (<= _output_get 0.0)
    (`self.OnGameOver`)
    (return true)
    (else
      (return false))))

(fn `HasEnoughResources`
  (params (ResourceAmount :type "/Game/Blueprints/F_ResourceAmount Structure"))
  (returns (HasEnough :type Boolean))
  (bind (_resources_magic _resources_metal) (break `/Game/Blueprints/F_ResourceAmount` (`self.Resources`)))
  (return (and (<= ResourceAmount_Magic_2_8E043D7A4642FD581AC3409B424337B5 _resources_magic) (<= ResourceAmount_Metal_4_9649F6DD4375FEB0841A53997C79FCCC _resources_metal))))

(fn `OnGameOver`)

(fn `SpendResources`
  (params (ResourceAmount :type "/Game/Blueprints/F_ResourceAmount Structure"))
  (returns (Success :type Boolean))
  (bind (_resources_magic _resources_metal) (break `/Game/Blueprints/F_ResourceAmount` (`self.Resources`)))
  (bind (_resourceamount_magic _resourceamount_metal) (break `/Game/Blueprints/F_ResourceAmount` (`local.ResourceAmount`)))
  (bind (_resourceamount_magic_2 _resourceamount_metal_2) (break `/Game/Blueprints/F_ResourceAmount` (`local.ResourceAmount`)))
  (if (`self.HasEnoughResources` ResourceAmount)
    (set `self.Resources` (make `/Game/Blueprints/F_ResourceAmount` (- _resources_magic _resourceamount_magic_2) (- _resources_metal _resourceamount_metal_2)))
    (`KismetSystemLibrary.PrintString` (`KismetStringLibrary.Concat_StrStr` "Spend " (`KismetStringLibrary.Conv_IntToString` _resourceamount_magic) " magic and " (`KismetStringLibrary.Conv_IntToString` _resourceamount_metal) " metal"))
    (return true)
    (else
      (return false))))

(fn `UserConstructionScript`)