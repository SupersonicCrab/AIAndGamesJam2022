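; Workshop interactable that builds a placeable for a chosen grid using its own construction robot, spawned on BeginPlay.
; Player AI interaction registers it on the player controller.
; Choosing a grid releases the previous lock, then, unless building, locks the new one, checks occupancy, resources and a synchronous nav path, spends the cost and flags the robot's blackboard ready.
; StartBuilding runs a timer that spawns the placeable and attaches it to the robot.
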(event `self.ReceiveBeginPlay`
  (`parent.ReceiveBeginPlay`)
  (`self.SpawnConstructionRobot`)
  (bind _asbp_game_mode (cast `/Game/Blueprints/BP_GameMode` (`GameplayStatics.GetGameMode`)))
  (set `self.GameMode` _asbp_game_mode))

(fn `CanReachGrid`
  (returns (bCanReach :type Boolean))
  (bind _returnvalue (`NavigationSystemV1.FindPathToActorSynchronously` (`self.K2_GetActorLocation`) (`self.Grid`) 50.0 null "/Game/NPCs/Navigation/NavFilter_ConstructionRobot.NavFilter_ConstructionRobot_C"))
  (return (not (`NavigationPath.IsPartial` _returnvalue))))

(fn `OnBuildComplete`
  (bind _returnvalue (`|SpawnActorFromClass` (`self.PlaceableClass`) (`KismetMathLibrary.MakeTransform` (0.0 0.0 0.0)) "Undefined" "OverrideRootScale" null null))
  (`/Game/NPCs/Robots/Construction/BP_ConstructionCharacter.AttachPlaceable` (`self.ConstructionRobot`) _returnvalue)
  (set `self.bBuilding` false))

(fn `OnGridChosen`
  (params (Grid :type "/Game/Blueprints/PlayArea/BP_Grid Object Reference"))
  (locals (GridName :type Name :default "Grid"))
  (bind _gamemode (`self.GameMode`))
  (bind _buildcost (`self.BuildCost`))
  (`self.UnlockGrid`)
  (if (not (`self.bBuilding`))
    (bind _output_get (set `self.Grid` Grid))
    (set `/Game/Blueprints/PlayArea/BP_Grid.bBuildLocked` true _output_get)
    (`/Game/Blueprints/PlayArea/BP_Grid.Placeable` Grid
      (:`then`
        (`self.SetReadyToBuild` false :!label _label))
      (:`else`
        (if (`/Game/Blueprints/BP_GameMode.HasEnoughResources` _gamemode _buildcost)
          (bind _bcanreach (`self.CanReachGrid`))
          (if _bcanreach
            (`/Game/Blueprints/BP_GameMode.SpendResources` _gamemode _buildcost)
            (`self.ConstructionRobot`
              (:`then`
                (`self.SetReadyToBuild` true))
              (:`else`
                (goto _label)))
            (else
              (goto _label)))
          (else
            (goto _label)))))))

(fn `OnPlayerAIInteraction`
  (params (PlayerController :type "/Game/Blueprints/Player/BP_PlayerController Object Reference") (PlayerAIController :type "/Game/Blueprints/Player/BP_PlayerAIController Object Reference"))
  (`parent.OnPlayerAIInteraction` PlayerController PlayerAIController)
  (set `/Game/Blueprints/Player/BP_PlayerController.PlaceableWorkshop` self PlayerController))

(fn `SetReadyToBuild`
  (params (ReadyToBuild :type Boolean))
  (locals (ReadyToBuildName :type Name :default "bReadyToBuild"))
  (bind _constructionrobot (`self.ConstructionRobot`)
    (:`then`
      (`BlackboardComponent.SetValueAsBool` (`/Game/NPCs/BP_NPCCharacter.Blackboard` _constructionrobot) (`local.ReadyToBuildName`) ReadyToBuild))
    (:`else`)))

(fn `SpawnConstructionRobot`
  (bind _returnvalue (`|SpawnActorFromClass` "/Game/NPCs/Robots/Construction/BP_ConstructionCharacter.BP_ConstructionCharacter_C" (`KismetMathLibrary.MakeTransform` (+ (`SceneComponent.K2_GetComponentLocation` (`self.ConstructionTransform`)) (0.0 0.0 200.0)) (struct :`Yaw` 180.0)) "AdjustIfPossibleButAlwaysSpawn" "OverrideRootScale" null null null))
  (bind _output_get (set `self.ConstructionRobot` _returnvalue))
  (`BlackboardComponent.SetValueAsObject` (`AIBlueprintHelperLibrary.GetBlackboard` _output_get) (`self.Workshop`) self)
  (set `/Game/NPCs/Robots/Construction/BP_ConstructionCharacter.PlaceableWorkshop` self _output_get))

(fn `StartBuilding`
  (`KismetSystemLibrary.K2_SetTimer` null "OnBuildComplete" (`self.BuildTime`))
  (set `self.bBuilding` true))

(fn `UnlockGrid`
  (bind _grid (`self.Grid`)
    (:`then`
      (set `/Game/Blueprints/PlayArea/BP_Grid.bBuildLocked` false _grid))
    (:`else`)))

(fn `UserConstructionScript`
  (`parent.UserConstructionScript`))