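; Robot workshop interactable that builds robots for a resource cost when a player's AI controller interacts with it.
; On interaction it spends the cost through BP_GameMode, then sets a build timer, flags itself as building and shows the crafting effect.
; When the timer ends, it spawns the configured robot class above the interaction transform, clears the flag and hides the effect.
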(event `self.ReceiveBeginPlay`
  (`parent.ReceiveBeginPlay`)
  (bind _asbp_game_mode (cast `/Game/Blueprints/BP_GameMode` (`GameplayStatics.GetGameMode`)))
  (set `self.GameMode` _asbp_game_mode))

(fn `OnBuildFinished`
  (bind _returnvalue (`SceneComponent.K2_GetComponentToWorld` (`self.InteractionTransform`)))
  (`|SpawnActorFromClass` (`self.RobotClass`) (`KismetMathLibrary.MakeTransform` (`KismetMathLibrary.MakeVector` (.x (.location _returnvalue)) (.y (.location _returnvalue)) (+ (.z (.location _returnvalue)) 150.0)) (.rotation _returnvalue) (.scale _returnvalue)) "AdjustIfPossibleButAlwaysSpawn" "OverrideRootScale" null null)
  (set `self.bBuilding` false)
  (`SceneComponent.SetVisibility` (`self.PFB_Crafting`) false false))

(fn `OnPlayerAIInteraction`
  (params (PlayerController :type "/Game/Blueprints/Player/BP_PlayerController Object Reference") (PlayerAIController :type "/Game/Blueprints/Player/BP_PlayerAIController Object Reference"))
  (`parent.OnPlayerAIInteraction` PlayerController PlayerAIController)
  (bind _success (`/Game/Blueprints/BP_GameMode.SpendResources` (`self.GameMode`) (`self.Cost`)))
  (if _success
    (`KismetSystemLibrary.K2_SetTimer` null "OnBuildFinished" (`self.BuildTime`))
    (set `self.bBuilding` true)
    (`SceneComponent.SetVisibility` (`self.PFB_Crafting`) true false)))

(fn `UserConstructionScript`
  (`parent.UserConstructionScript`))