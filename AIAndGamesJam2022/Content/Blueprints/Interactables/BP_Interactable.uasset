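; BP_Interactable is a Blueprint for objects that a player and their AI controller can interact with.
; OnPlayerAIInteraction stores the PlayerController when an interaction begins, and OnPlayerAIInteractionFinished clears it when the interaction ends.
; Both functions print the player and AI controller names as debug output, with no further interaction behavior.
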(fn `OnPlayerAIInteraction`
  (params (PlayerController :type "/Game/Blueprints/Player/BP_PlayerController Object Reference") (PlayerAIController :type "/Game/Blueprints/Player/BP_PlayerAIController Object Reference"))
  (`KismetSystemLibrary.PrintString` (`KismetStringLibrary.Concat_StrStr` (`KismetSystemLibrary.GetDisplayName` PlayerController) (`KismetSystemLibrary.GetDisplayName` PlayerAIController)))
  (set `self.PlayerController` PlayerController))

(fn `OnPlayerAIInteractionFinished`
  (params (PlayerController :type "/Game/Blueprints/Player/BP_PlayerController Object Reference") (PlayerAIController :type "/Game/Blueprints/Player/BP_PlayerAIController Object Reference"))
  (`KismetSystemLibrary.PrintString` (`KismetStringLibrary.Concat_StrStr` (`KismetSystemLibrary.GetDisplayName` PlayerController) (`KismetSystemLibrary.GetDisplayName` PlayerAIController)))
  (set `self.PlayerController` null))

(fn `UserConstructionScript`)