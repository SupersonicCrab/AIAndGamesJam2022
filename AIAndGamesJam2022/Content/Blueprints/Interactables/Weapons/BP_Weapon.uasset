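; Base-style interactable weapon that the player aims at the cursor while an interaction is active, with heat-limited firing.
; Each tick decays heat and, while Firing, attempts a shot, which requires aiming, an in-play-area target and enough heat headroom.
; A shot only prints its aim location, adds heat and starts a cooldown timer that restores ReadyToFire, though the firing check never reads that flag.
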(event `self.ReceiveTick`
  (params (DeltaSeconds :type "Float (single-precision)"))
  (`parent.ReceiveTick` DeltaSeconds)
  (`self.DecayHeat`)
  (if (`self.bFiring`)
    (`self.OnWeaponFired`)))

(fn `DecayHeat`
  (set `self.Heat` (`KismetMathLibrary.FClamp` (- (`self.Heat`) (* (`self.HeatDecayRate`) (`GameplayStatics.GetWorldDeltaSeconds`))) 0.0 (`self.MaxHeat`))))

(fn `OnCooldownFinished`
  (set `self.bReadyToFire` true))

(fn `OnPlayerAIInteraction`
  (params (PlayerController :type "/Game/Blueprints/Player/BP_PlayerController Object Reference") (PlayerAIController :type "/Game/Blueprints/Player/BP_PlayerAIController Object Reference"))
  (`parent.OnPlayerAIInteraction` PlayerController PlayerAIController)
  (set `self.bAiming` true))

(fn `OnPlayerAIInteractionFinished`
  (params (PlayerController :type "/Game/Blueprints/Player/BP_PlayerController Object Reference") (PlayerAIController :type "/Game/Blueprints/Player/BP_PlayerAIController Object Reference"))
  (`parent.OnPlayerAIInteractionFinished` PlayerController PlayerAIController)
  (set `self.bAiming` false))

(fn `OnWeaponFired`
  (returns (bWeaponFired :type Boolean))
  (bind (_aimlocation _bwithinplayarea) (`/Game/Blueprints/Player/BP_PlayerController.GetCursorAimLocation` (`self.PlayerController`)))
  (`|ExecutionSequence`
    (:`then_0`
      (if (`self.bAiming`)
        (set `self.AimLocation` _aimlocation)
        (if _bwithinplayarea
          (if (and (< (`self.Heat`) (`self.MaxHeat`)) (>= (- (`self.MaxHeat`) (`self.Heat`)) (`self.HeatIncreaseRate`)))
            (`KismetSystemLibrary.PrintString` (`KismetStringLibrary.Concat_StrStr` "Fired at " (`KismetStringLibrary.Conv_VectorToString` (`self.AimLocation`))))
            (set `self.bReadyToFire` false)
            (set `self.Heat` (`KismetMathLibrary.FClamp` (+ (`self.Heat`) (`self.HeatIncreaseRate`)) 0.0 (`self.MaxHeat`)))
            (`KismetSystemLibrary.K2_SetTimer` null "OnCooldownFinished" (`self.ShotCooldown`))
            (return true)
            (else
              (`KismetSystemLibrary.PrintString` "Too hot!" true true (struct :`G` 0.66 :`B` 1.0 :`A` 1.0) 0.0)))
          (else
            (`KismetSystemLibrary.PrintString` "Not in play area!" true true (struct :`G` 0.66 :`B` 1.0 :`A` 1.0) 0.0)))))
    (:`then_1`
      (return false))))

(fn `UserConstructionScript`
  (`parent.UserConstructionScript`))