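; Harpoon projectile that collects resources around the point where it strikes.
; Each tick it pitches its mesh to follow the velocity.
; On mesh hit it draws a debug sphere, finds WorldStatic BP_Resource actors within Range and passes each to GM_DwarfStuck's CollectResource.
; It then destroys itself.
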(event `self.ReceiveBeginPlay`
  (`parent.ReceiveBeginPlay`)
  (bind _asgm_dwarf_stuck (cast `/Game/Blueprints/GM_DwarfStuck` (`GameplayStatics.GetGameMode`)))
  (set `self.GameMode` _asgm_dwarf_stuck))

(event `self.ReceiveTick`
  (params (DeltaSeconds :type "Float (single-precision)"))
  (bind _staticmesh (`self.StaticMesh`))
  (bind (_returnvalue_roll _returnvalue_pitch) (`KismetMathLibrary.BreakRotator` (`KismetMathLibrary.Conv_VectorToRotator` (`self.GetVelocity`))))
  (bind (_relativerotation_roll _relativerotation_pitch _relativerotation_yaw) (`KismetMathLibrary.BreakRotator` (`SceneComponent.RelativeRotation` _staticmesh)))
  (`parent.ReceiveTick` DeltaSeconds)
  (`SceneComponent.K2_SetRelativeRotation` _staticmesh (`KismetMathLibrary.MakeRotator` _relativerotation_roll _returnvalue_pitch _relativerotation_yaw) false true))

(event `self.StaticMesh.OnComponentHit`
  (params (HitComponent :type "PrimitiveComponent Object Reference") (OtherActor :type "Actor Object Reference") (OtherComp :type "PrimitiveComponent Object Reference") (NormalImpulse :type "Vector Structure") (Hit :type "HitResult Structure (by ref)"))
  (bind _returnvalue (`self.K2_GetActorLocation`))
  (bind _range (`self.Range`))
  (`|ExecutionSequence`
    (:`then_0`
      (`KismetSystemLibrary.DrawDebugSphere` _returnvalue _range 12 (struct :`R` 1.0 :`G` 1.0 :`B` 1.0 :`A` 1.0) 5.0 1.0)
      (bind _outactors (`KismetSystemLibrary.SphereOverlapActors` _returnvalue _range (`|MakeArray` "ObjectTypeQuery1" :!type "EObjectTypeQuery Enum") "/Game/Blueprints/Resources/BP_Resource.BP_Resource_C"))
      (for _array_element _outactors
        (bind _asbp_resource (cast `/Game/Blueprints/Resources/BP_Resource` _array_element))
        (`/Game/Blueprints/GM_DwarfStuck.CollectResource` (`self.GameMode`) _asbp_resource)))
    (:`then_1`
      (`self.K2_DestroyActor`))))

(fn `UserConstructionScript`
  (`parent.UserConstructionScript`))