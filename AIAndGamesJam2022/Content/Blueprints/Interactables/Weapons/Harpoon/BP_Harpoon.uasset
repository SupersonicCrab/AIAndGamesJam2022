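; BP_Harpoon is a harpoon weapon that launches a projectile when fired.
; When the parent's fire logic succeeds, it spawns the projectile class at the ProjectileSpawn transform and applies the toss velocity to its static mesh as a velocity-change impulse.
; It then makes the ProjectileProxy component visible.
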(fn `OnWeaponFired`
  (bind _bweaponfired (`parent.OnWeaponFired`))
  (if _bweaponfired
    (bind _returnvalue (`|SpawnActorFromClass` (`self.ProjectileClass`) (`SceneComponent.K2_GetComponentToWorld` (`self.ProjectileSpawn`)) "Undefined" "OverrideRootScale" null null))
    (`PrimitiveComponent.AddImpulse` (`/Game/Blueprints/Interactables/Weapons/BP_Projectile.StaticMesh` _returnvalue) (`self.TossVelocity`) "None" true)
    (`SceneComponent.SetVisibility` (`self.ProjectileProxy`) true false)))

(fn `UserConstructionScript`
  (`parent.UserConstructionScript`))