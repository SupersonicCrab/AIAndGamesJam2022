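; BP_ProjectileWeapon is an interactable weapon that turns its mount to match a ballistic arc toward the aim point when fired.
; It overrides OnWeaponFired, calling the parent first, then, if aiming, yawing Base toward AimLocation.
; It pitches Turret from a suggested projectile velocity at LaunchSpeed, computed without tracing and converted to actor space.
; No projectile spawning happens here, and the parent's result is returned.
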(fn `OnWeaponFired`
  (returns (bWeaponFired :type Boolean))
  (bind _returnvalue (`self.K2_GetActorLocation`))
  (bind (_returnvalue_roll _returnvalue_pitch _returnvalue_yaw) (`KismetMathLibrary.BreakRotator` (`KismetMathLibrary.FindLookAtRotation` _returnvalue (`self.AimLocation`))))
  (bind _bweaponfired (`parent.OnWeaponFired`))
  (`|ExecutionSequence`
    (:`then_0`
      (if (`self.bAiming`)
        (`SceneComponent.K2_SetWorldRotation` (`self.Base`) (`KismetMathLibrary.MakeRotator` 0.0 0.0 _returnvalue_yaw) false false)
        (bind _tossvelocity (`GameplayStatics.BlueprintSuggestProjectileVelocity` _returnvalue (`self.AimLocation`) (`self.LaunchSpeed`) 0.0 "DoNotTrace"))
        (bind _output_get (set `self.TossVelocity` _tossvelocity))
        (bind (_returnvalue_roll_2 _returnvalue_pitch_2) (`KismetMathLibrary.BreakRotator` (`KismetMathLibrary.InverseTransformRotation` (`self.GetTransform`) (`KismetMathLibrary.Conv_VectorToRotator` _output_get))))
        (`SceneComponent.K2_SetRelativeRotation` (`self.Turret`) (`KismetMathLibrary.MakeRotator` 0.0 _returnvalue_pitch_2) false false)))
    (:`then_1`
      (return _bweaponfired))))

(fn `UserConstructionScript`
  (`parent.UserConstructionScript`))