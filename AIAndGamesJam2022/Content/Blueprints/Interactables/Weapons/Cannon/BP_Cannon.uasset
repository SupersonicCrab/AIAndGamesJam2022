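; Cannon weapon Blueprint that lobs a physics projectile along an arc toward its aim location.
; When the parent fire check succeeds, it snaps the base's yaw toward the target and pitches the turret to match the computed launch velocity.
; It then spawns the projectile at the spawn component and launches its mesh with a mass-independent impulse from SuggestProjectileVelocityCustomArc.
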(fn `OnWeaponFired`
  (bind _returnvalue (`self.K2_GetActorLocation`))
  (bind _aimlocation (`self.AimLocation`))
  (bind (_returnvalue_roll _returnvalue_pitch _returnvalue_yaw) (`KismetMathLibrary.BreakRotator` (`KismetMathLibrary.FindLookAtRotation` _returnvalue _aimlocation)))
  (bind _bweaponfired (`parent.OnWeaponFired`))
  (if _bweaponfired
    (`SceneComponent.K2_SetWorldRotation` (`self.Base`) (`KismetMathLibrary.MakeRotator` 0.0 0.0 _returnvalue_yaw) false false)
    (bind _outlaunchvelocity (`GameplayStatics.SuggestProjectileVelocity_CustomArc` _returnvalue _aimlocation 0.0 0.7))
    (bind (_returnvalue_roll_2 _returnvalue_pitch_2) (`KismetMathLibrary.BreakRotator` (`KismetMathLibrary.InverseTransformRotation` (`self.GetTransform`) (`KismetMathLibrary.Conv_VectorToRotator` _outlaunchvelocity))))
    (`SceneComponent.K2_SetRelativeRotation` (`self.Turret`) (`KismetMathLibrary.MakeRotator` 0.0 _returnvalue_pitch_2) false false)
    (bind _returnvalue_2 (`|SpawnActorFromClass` (`self.ProjectileClass`) (`SceneComponent.K2_GetComponentToWorld` (`self.ProjectileSpawn`)) "Undefined" "OverrideRootScale" null null))
    (`PrimitiveComponent.AddImpulse` (`/Game/Blueprints/Interactables/Weapons/BP_Projectile.StaticMesh` _returnvalue_2) _outlaunchvelocity "None" true)))

(fn `UserConstructionScript`
  (`parent.UserConstructionScript`))