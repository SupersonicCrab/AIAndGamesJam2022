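; BP_CharacterSpawner is an actor that spawns a character of a configurable class at its own transform.
; BeginPlay spawns automatically when SpawnOnBeginplay is set, using the configured collision handling override.
; SpawnCharacter returns the new actor, and SpawnCharacterByClass overwrites the stored class before calling it, so later spawns also use that class.
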(event `self.ReceiveBeginPlay`
  (if (`self.bSpawnOnBeginplay`)
    (`self.SpawnCharacter`)))

(fn `SpawnCharacter`
  (returns (SpawnedActor :type "Actor Object Reference"))
  (bind _returnvalue (`|SpawnActorFromClass` (`self.CharacterClass`) (`self.GetTransform`) (`self.CollisionHandlingOverride`) "OverrideRootScale" null null))
  (return _returnvalue))

(fn `SpawnCharacterByClass`
  (params (CharacterClass :type "Character Class Reference"))
  (returns (SpawnedActor :type "Actor Object Reference"))
  (set `self.CharacterClass` CharacterClass)
  (bind _spawnedactor (`self.SpawnCharacter`))
  (return _spawnedactor))

(fn `UserConstructionScript`)