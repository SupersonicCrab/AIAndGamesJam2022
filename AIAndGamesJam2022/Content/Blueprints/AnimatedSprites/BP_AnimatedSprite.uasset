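; Animated sprite actor that plays a Paper2D flipbook and can remove itself when playback finishes.
; With DestroyAfterPlaying set, BeginPlay turns off looping and the finished-playing event destroys the actor.
; FaceCamera runs only from the construction script, setting roll from a look-at toward the player camera plus an offset, yaw from the offset alone, and keeping pitch.
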(event `self.ReceiveBeginPlay`
  (`parent.ReceiveBeginPlay`)
  (if (`self.bDestroyAfterPlaying`)
    (`PaperFlipbookComponent.SetLooping` (`self.PaperFlipbook`) false)))

(event `self.PaperFlipbook.OnFinishedPlaying`
  (if (`self.bDestroyAfterPlaying`)
    (`self.K2_DestroyActor`)))

(fn `FaceCamera`
  (locals (Offset :type "Rotator Structure" :default (struct :`Yaw` 90.0 :`Roll` -40.0)))
  (bind _paperflipbook (`self.PaperFlipbook`))
  (bind (_offset_roll _offset_pitch _offset_yaw) (`KismetMathLibrary.BreakRotator` (`local.Offset`)))
  (bind (_returnvalue_roll _returnvalue_pitch) (`KismetMathLibrary.BreakRotator` (`SceneComponent.K2_GetComponentRotation` _paperflipbook)))
  (bind _returnvalue_roll_2 (`KismetMathLibrary.BreakRotator` (`KismetMathLibrary.FindLookAtRotation` (`self.K2_GetActorLocation`) (`PlayerCameraManager.GetCameraLocation` (`GameplayStatics.GetPlayerCameraManager` 0)))))
  (`SceneComponent.K2_SetWorldRotation` _paperflipbook (`KismetMathLibrary.MakeRotator` (+ _returnvalue_roll_2 _offset_roll) _returnvalue_pitch _offset_yaw) false false))

(fn `UserConstructionScript`
  (`self.FaceCamera`))