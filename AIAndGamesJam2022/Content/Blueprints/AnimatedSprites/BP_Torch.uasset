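; BP_Torch is an animated torch sprite that periodically mirrors its Paper2D flipbook.
; On BeginPlay it reads the flipbook length and starts a looping timer at that length times FlipRatio.
; Each timer tick calls FlipSprite, which negates the flipbook component's X scale to flip it horizontally, varying the looping animation.
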(event `self.ReceiveBeginPlay`
  (`parent.ReceiveBeginPlay`)
  (bind _output_get (set `self.FlipbookLength` (`PaperFlipbookComponent.GetFlipbookLength` (`self.PaperFlipbook`))))
  (`KismetSystemLibrary.K2_SetTimer` null "FlipSprite" (* _output_get (`self.FlipRatio`)) true))

(fn `FlipSprite`
  (bind _paperflipbook (`self.PaperFlipbook`))
  (bind (_relativescale3d_x _relativescale3d_y _relativescale3d_z) (`KismetMathLibrary.BreakVector` (`SceneComponent.RelativeScale3D` _paperflipbook)))
  (`SceneComponent.SetRelativeScale3D` _paperflipbook (`KismetMathLibrary.MakeVector` (* _relativescale3d_x -1.0) _relativescale3d_y _relativescale3d_z)))

(fn `UserConstructionScript`
  (`parent.UserConstructionScript`))