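; Sprite Blueprint that orients its PaperSprite relative to the first player's camera through a FaceCamera function.
; The construction script calls FaceCamera, with no per-frame update in the graphs, and rotation is skipped without a valid camera manager.
; Only the look-at rotation's roll is used, added to the Offset roll, while pitch is preserved and yaw comes solely from Offset.
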(fn `FaceCamera`
  (locals (Offset :type "Rotator Structure" :default (struct :`Yaw` 90.0 :`Roll` -40.0)))
  (bind _returnvalue (`GameplayStatics.GetPlayerCameraManager` 0))
  (bind (_offset_roll _offset_pitch _offset_yaw) (`KismetMathLibrary.BreakRotator` (`local.Offset`)))
  (bind (_returnvalue_roll _returnvalue_pitch) (`KismetMathLibrary.BreakRotator` (`SceneComponent.K2_GetComponentRotation` (`self.PaperSprite`))))
  (bind _returnvalue_roll_2 (`KismetMathLibrary.BreakRotator` (`KismetMathLibrary.FindLookAtRotation` (`self.K2_GetActorLocation`) (`PlayerCameraManager.GetCameraLocation` _returnvalue))))
  (`/Engine/EditorBlueprintResources/StandardMacros.IsValid` _returnvalue
    (:`Is Valid`
      (`SceneComponent.K2_SetWorldRotation` (`self.PaperSprite`) (`KismetMathLibrary.MakeRotator` (+ _returnvalue_roll_2 _offset_roll) _returnvalue_pitch _offset_yaw) false false))))

(fn `UserConstructionScript`
  (`self.FaceCamera`))