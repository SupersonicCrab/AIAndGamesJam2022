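; BP_Explosion is an explosion actor that damages nearby enemies as soon as it spawns.
; On BeginPlay it runs its parent logic, plays the explosion sound and draws a debug sphere showing its Range.
; A sphere overlap gathers BP_EnemyCharacter pawns, and each one whose actor distance is under Range takes Damage, with the explosion as damage causer.
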(event `self.ReceiveBeginPlay`
  (bind _returnvalue (`self.K2_GetActorLocation`))
  (bind _range (`self.Range`))
  (`parent.ReceiveBeginPlay`)
  (`GameplayStatics.PlaySoundAtLocation` "/Game/Assets/Audio/Effects/A_Explosion.A_Explosion" (`self.K2_GetActorLocation`) (struct) 1.0 1.0 0.0 null null null null)
  (`KismetSystemLibrary.DrawDebugSphere` _returnvalue _range 12 (struct :`R` 1.0 :`G` 1.0 :`B` 1.0 :`A` 1.0) 5.0 1.0)
  (bind _outactors (`KismetSystemLibrary.SphereOverlapActors` _returnvalue _range (`|MakeArray` "ObjectTypeQuery3" :!type "EObjectTypeQuery Enum") "/Game/NPCs/Enemies/BP_EnemyCharacter.BP_EnemyCharacter_C"))
  (for _array_element _outactors
    (if (< (`self.GetDistanceTo` _array_element) (`self.Range`))
      (`GameplayStatics.ApplyDamage` _array_element (`self.Damage`) null self))))

(fn `UserConstructionScript`
  (`parent.UserConstructionScript`))