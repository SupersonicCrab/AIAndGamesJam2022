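; Paper2D sprite character that orients its sprite toward the camera and picks its look from facing relative to the camera.
; Tick adjusts sprite rotation and compares camera and actor vectors, choosing Up or Down sprites by action name from a map and mirroring X scale for left/right.
; A MovementAnimation timeline, started after a random delay with random sway direction, defines speed-scaled sway, bob and play rate, with a separate rate while falling.
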(event `self.ReceiveTick`
  (params (DeltaSeconds :type "Float (single-precision)"))
  (`parent.ReceiveTick` DeltaSeconds)
  (`self.FaceCamera`)
  (`self.UpdateLookDirection`)
  (`SceneComponent.K2_SetRelativeLocation` (`self.PaperSprite`) (`KismetMathLibrary.MakeVector` 0.0 0.0 (* (`CapsuleComponent.CapsuleHalfHeight` (`self.CapsuleComponent`)) -1.0)) false true))

(event `self.ReceiveBeginPlay`
  (`parent.ReceiveBeginPlay`)
  (set `self.PlayerCameraManager` (`GameplayStatics.GetPlayerCameraManager` 0))
  (set `self.SwayFlip` (`KismetMathLibrary.RandomBoolFromStream` (`KismetMathLibrary.MakeRandomStream` (`KismetMathLibrary.RandomInteger` 2048))))
  (`KismetSystemLibrary.Delay` (`KismetMathLibrary.RandomFloatInRange` 0.0 0.5))
  (`TimelineComponent.PlayFromStart` (`self.MovementAnimation`)))

(fn `FaceCamera`
  (locals (Offset :type "Rotator Structure" :default (struct :`Yaw` 90.0 :`Roll` -20.0)))
  (bind (_offset_roll _offset_pitch _offset_yaw) (`KismetMathLibrary.BreakRotator` (`local.Offset`)))
  (bind (_returnvalue_roll _returnvalue_pitch) (`KismetMathLibrary.BreakRotator` (`SceneComponent.K2_GetComponentRotation` (`self.PaperSprite`))))
  (bind _returnvalue_roll_2 (`KismetMathLibrary.BreakRotator` (`KismetMathLibrary.FindLookAtRotation` (`self.K2_GetActorLocation`) (`PlayerCameraManager.GetCameraLocation` (`GameplayStatics.GetPlayerCameraManager` 0)))))
  (`SceneComponent.K2_SetWorldRotation` (`self.PaperSprite`) (`KismetMathLibrary.MakeRotator` (+ _returnvalue_roll_2 _offset_roll) _returnvalue_pitch _offset_yaw) false false))

(fn `UpdateLookDirection`
  (bind _returnvalue (> (`KismetMathLibrary.Dot_VectorVector` (`self.GetActorForwardVector` (`self.PlayerCameraManager`)) (`self.GetActorForwardVector`)) 0.0))
  (bind _returnvalue_2 (> (`KismetMathLibrary.Dot_VectorVector` (`self.GetActorRightVector` (`self.PlayerCameraManager`)) (`self.GetActorForwardVector`)) 0.0))
  (`self.PlayerCameraManager`
    (:`then`
      (`|ExecutionSequence`
        (:`then_0`
          (if (!= _returnvalue (`self.bLookingUp`))
            (set `self.bLookingUp` _returnvalue)
            (`self.UpdateSprite` (`self.CurrentSpriteAction`))))
        (:`then_1`
          (if (!= _returnvalue_2 (`self.bLookingRight`))
            (bind _output_get (set `self.bLookingRight` _returnvalue_2))
            (`SceneComponent.SetRelativeScale3D` (`self.PaperSprite`) (`KismetMathLibrary.MakeVector` (select `bool` _output_get :`false` -1.0 :`true` 1.0) 1.0 1.0))))))
    (:`else`)))

(fn `UpdateSprite`
  (params (ActionName :type String))
  (set `self.CurrentSpriteAction` ActionName)
  (`PaperSpriteComponent.SetSprite` (`self.PaperSprite`) (`BlueprintMapLibrary.Map_Find` (`self.Sprites`) (`KismetStringLibrary.Conv_StringToName` (`KismetStringLibrary.Concat_StrStr` (select `bool` (`self.bLookingUp`) :`false` "Down" :`true` "Up") ActionName)))))

(fn `UserConstructionScript`
  (`self.UpdateSprite` ""))