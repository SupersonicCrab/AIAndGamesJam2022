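; Game mode for DwarfStuck that owns shared health, the Magic and Metal resources, and per-class sound volume settings.
; Game start blends the view to the player camera and starts wave 1 on the wave manager.
; Resource changes and damage broadcast update events, while healing only clamps and prints; zero health triggers game lost, which, like game won, only prints.
; BeginPlay applies the stored Master, Music and SFX volumes through sound mix overrides.
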(event `self.ReceiveBeginPlay`
  (`parent.ReceiveBeginPlay`)
  (`self.SetupVolume`))

(fn `AddResources`
  (params (ResourcesToAdd :type "/Game/Blueprints/F_ResourceAmount Structure"))
  (bind (_resources_magic _resources_metal) (break `/Game/Blueprints/F_ResourceAmount` (`self.Resources`)))
  (bind _output_get (set `self.Resources` (make `/Game/Blueprints/F_ResourceAmount` (+ _resources_magic ResourcesToAdd_Magic_2_8E043D7A4642FD581AC3409B424337B5) (+ _resources_metal ResourcesToAdd_Metal_4_9649F6DD4375FEB0841A53997C79FCCC))))
  (`self.OnResourcesUpdated` _output_get))

(fn `CollectResource`
  (params (Resource :type "/Game/Blueprints/Resources/BP_Resource Object Reference"))
  (bind (_resourcesgained_magic _resourcesgained_metal) (break `/Game/Blueprints/F_ResourceAmount` (`/Game/Blueprints/Resources/BP_Resource.ResourcesGained` Resource)))
  (bind (_resources_magic _resources_metal) (break `/Game/Blueprints/F_ResourceAmount` (`self.Resources`)))
  (bind _output_get (set `self.Resources` (make `/Game/Blueprints/F_ResourceAmount` (+ _resources_magic _resourcesgained_magic) (+ _resources_metal _resourcesgained_metal))))
  (`self.OnResourcesUpdated` _output_get)
  (`/Game/Blueprints/Resources/BP_Resource.OnResourceDestroyed` Resource))

(fn `DealDamage`
  (params (Damage :type "Float (double-precision)"))
  (returns (bLost :type Boolean))
  (bind _output_get (set `self.Health` (`KismetMathLibrary.FClamp` (- (`self.Health`) Damage) 0.0 (`.Health` (defaults `/Game/Blueprints/GM_DwarfStuck` "GM_DwarfStuck_C")))))
  (`self.HealthUpdated` _output_get)
  (if (<= _output_get 0.0)
    (`self.OnGameLost`)
    (return true)
    (else
      (return false))))

(fn `GetVolume`
  (params (SoundClass :type "SoundClass Object Reference"))
  (returns (Volume :type "Float (double-precision)") (bVolumeFound :type Boolean))
  (bind (_value _returnvalue) (`BlueprintMapLibrary.Map_Find` (`self.SoundSettings`) SoundClass))
  (return _value _returnvalue))

(fn `HasEnoughResources`
  (params (ResourceAmount :type "/Game/Blueprints/F_ResourceAmount Structure"))
  (returns (HasEnough :type Boolean))
  (bind (_resources_magic _resources_metal) (break `/Game/Blueprints/F_ResourceAmount` (`self.Resources`)))
  (return (and (<= ResourceAmount_Magic_2_8E043D7A4642FD581AC3409B424337B5 _resources_magic) (<= ResourceAmount_Metal_4_9649F6DD4375FEB0841A53997C79FCCC _resources_metal))))

(fn `Heal`
  (params (Amount :type "Float (double-precision)"))
  (set `self.Health` (`KismetMathLibrary.FClamp` (+ (`self.Health`) Amount) 0.0 (`.Health` (defaults `/Game/Blueprints/GM_DwarfStuck` "GM_DwarfStuck_C"))))
  (`KismetSystemLibrary.PrintString` (`KismetStringLibrary.Concat_StrStr` "Healed for " (`KismetStringLibrary.Conv_DoubleToString` (`local.Amount`)))))

(fn `OnGameLost`
  (`KismetSystemLibrary.PrintString` "Game lost"))

(fn `OnGameStarted`
  (bind _returnvalue (`GameplayStatics.GetActorOfClass` "/Game/Blueprints/Player/BP_PlayerCamera.BP_PlayerCamera_C"))
  (`PlayerController.SetViewTargetWithBlend` (`GameplayStatics.GetPlayerController` 0) _returnvalue 3.0 "VTBlend_Linear" 0.0 false)
  (bind _returnvalue_2 (`GameplayStatics.GetActorOfClass` "/Game/NPCs/WaveManger/BP_WaveManager.BP_WaveManager_C"))
  (`/Game/NPCs/WaveManger/BP_WaveManager.StartWave` _returnvalue_2 1))

(fn `OnGameWon`
  (`KismetSystemLibrary.PrintString` "Game won"))

(fn `SetupVolume`
  (`self.UpdateVolume` "/Game/Assets/Audio/SoundClasses/S_Master.S_Master" (`BlueprintMapLibrary.Map_Find` (`self.SoundSettings`) "/Game/Assets/Audio/SoundClasses/S_Master.S_Master"))
  (`self.UpdateVolume` "/Game/Assets/Audio/SoundClasses/S_Music.S_Music" (`BlueprintMapLibrary.Map_Find` (`self.SoundSettings`) "/Game/Assets/Audio/SoundClasses/S_Music.S_Music"))
  (`self.UpdateVolume` "/Game/Assets/Audio/SoundClasses/S_SFX.S_SFX" (`BlueprintMapLibrary.Map_Find` (`self.SoundSettings`) "/Game/Assets/Audio/SoundClasses/S_SFX.S_SFX")))

(fn `SpendResources`
  (params (ResourceAmount :type "/Game/Blueprints/F_ResourceAmount Structure"))
  (returns (Success :type Boolean))
  (bind (_resources_magic _resources_metal) (break `/Game/Blueprints/F_ResourceAmount` (`self.Resources`)))
  (bind (_resourceamount_magic _resourceamount_metal) (break `/Game/Blueprints/F_ResourceAmount` (`local.ResourceAmount`)))
  (bind (_resourceamount_magic_2 _resourceamount_metal_2) (break `/Game/Blueprints/F_ResourceAmount` (`local.ResourceAmount`)))
  (if (`self.HasEnoughResources` ResourceAmount)
    (bind _output_get (set `self.Resources` (make `/Game/Blueprints/F_ResourceAmount` (- _resources_magic _resourceamount_magic_2) (- _resources_metal _resourceamount_metal_2))))
    (`self.OnResourcesUpdated` _output_get)
    (`KismetSystemLibrary.PrintString` (`KismetStringLibrary.Concat_StrStr` "Spent " (`KismetStringLibrary.Conv_IntToString` _resourceamount_magic) " magic and " (`KismetStringLibrary.Conv_IntToString` _resourceamount_metal) " metal"))
    (return true)
    (else
      (return false))))

(fn `UpdateVolume`
  (params (SoundClass :type "SoundClass Object Reference") (NewVolume :type "Float (double-precision)"))
  (locals (FadeInTime :type "Float (single-precision)" :default 0.0))
  (`BlueprintMapLibrary.Map_Add` (`self.SoundSettings`) SoundClass NewVolume)
  (`GameplayStatics.SetSoundMixClassOverride` "/Game/Assets/Audio/SoundClasses/MasterMix.MasterMix" (`local.SoundClass`) (`local.NewVolume`) 1.0 (`local.FadeInTime`))
  (`GameplayStatics.PushSoundMixModifier` "/Game/Assets/Audio/SoundClasses/MasterMix.MasterMix"))

(fn `UserConstructionScript`)