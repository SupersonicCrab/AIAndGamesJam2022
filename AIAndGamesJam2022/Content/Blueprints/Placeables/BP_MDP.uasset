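; BP_MDP is a placeable area device that slows and steadily damages enemies inside its sphere.
; Sphere overlaps track each BP_EnemyCharacter, scaling its walk speed by SlowRatio on entry and restoring the default on exit.
; Tick spins the mesh and applies frame-time-scaled damage to every tracked enemy.
; When placed, it adds a second sphere sized from the first by AvoidRatio.
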(event `self.Sphere.OnComponentBeginOverlap`
  (params (OverlappedComponent :type "PrimitiveComponent Object Reference") (OtherActor :type "Actor Object Reference") (OtherComp :type "PrimitiveComponent Object Reference") (OtherBodyIndex :type Integer) (bFromSweep :type Boolean) (SweepResult :type "HitResult Structure (by ref)"))
  (bind _asbp_enemy_character (cast `/Game/NPCs/Enemies/BP_EnemyCharacter` OtherActor))
  (`KismetArrayLibrary.Array_Add` (`self.TrackedEnemies`) _asbp_enemy_character)
  (`self.UpdateEnemySpeed` _asbp_enemy_character (`self.SlowRatio`)))

(event `self.Sphere.OnComponentEndOverlap`
  (params (OverlappedComponent :type "PrimitiveComponent Object Reference") (OtherActor :type "Actor Object Reference") (OtherComp :type "PrimitiveComponent Object Reference") (OtherBodyIndex :type Integer))
  (bind _asbp_enemy_character (cast `/Game/NPCs/Enemies/BP_EnemyCharacter` OtherActor))
  (`KismetArrayLibrary.Array_RemoveItem` (`self.TrackedEnemies`) _asbp_enemy_character)
  (`self.RestoreEnemySpeed` _asbp_enemy_character))

(event `self.ReceiveTick`
  (params (DeltaSeconds :type "Float (single-precision)"))
  (`parent.ReceiveTick` DeltaSeconds)
  (`SceneComponent.K2_AddRelativeRotation` (`self.StaticMesh`) (* (`self.RotationDelta`) DeltaSeconds) false false)
  (for _array_element (`self.TrackedEnemies`)
    (`GameplayStatics.ApplyDamage` _array_element (* DeltaSeconds (`self.Damage`)) null self)))

(fn `OnPlaced`
  (`parent.OnPlaced`)
  (bind _returnvalue (`AddComponent|NODE_AddSphereComponent-0`))
  (`SphereComponent.SetSphereRadius` _returnvalue (* (`SphereComponent.SphereRadius` (`self.Sphere`)) (`self.AvoidRatio`)) true))

(fn `RestoreEnemySpeed`
  (params (Enemy :type "/Game/NPCs/Enemies/BP_EnemyCharacter Object Reference"))
  (set `CharacterMovementComponent.MaxWalkSpeed` (`/Game/NPCs/Enemies/BP_EnemyCharacter.DefaultWalkSpeed` Enemy) (`Character.CharacterMovement` Enemy)))

(fn `UpdateEnemySpeed`
  (params (Enemy :type "/Game/NPCs/Enemies/BP_EnemyCharacter Object Reference") (NewRate :type "Float (double-precision)"))
  (set `CharacterMovementComponent.MaxWalkSpeed` (* NewRate (`/Game/NPCs/Enemies/BP_EnemyCharacter.DefaultWalkSpeed` Enemy)) (`Character.CharacterMovement` Enemy)))

(fn `UserConstructionScript`
  (`parent.UserConstructionScript`))