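; BP_Mine is a placeable mine that explodes when a BP_EnemyCharacter begins overlapping its Sphere component.
; On trigger, it runs a sphere overlap query at its location using Range and applies Damage to each enemy found, drawing a debug sphere of that radius.
; It then spawns BP_Explosion slightly offset along world X and destroys itself.
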(event `self.Sphere.OnComponentBeginOverlap`
  (params (OverlappedComponent :type "PrimitiveComponent Object Reference") (OtherActor :type "Actor Object Reference") (OtherComp :type "PrimitiveComponent Object Reference") (OtherBodyIndex :type Integer) (bFromSweep :type Boolean) (SweepResult :type "HitResult Structure (by ref)"))
  (bind _returnvalue (`self.K2_GetActorLocation`))
  (bind (_returnvalue_x _returnvalue_y _returnvalue_z) (`KismetMathLibrary.BreakVector` (`self.K2_GetActorLocation`)))
  (bind _range (`self.Range`))
  (cast `/Game/NPCs/Enemies/BP_EnemyCharacter` OtherActor)
  (`|ExecutionSequence`
    (:`then_0`
      (`KismetSystemLibrary.DrawDebugSphere` _returnvalue _range 12 (struct :`R` 1.0 :`G` 1.0 :`B` 1.0 :`A` 1.0) 1.0 1.0)
      (bind _outactors (`KismetSystemLibrary.SphereOverlapActors` _returnvalue _range (`|MakeArray` "ObjectTypeQuery3" :!type "EObjectTypeQuery Enum") "/Game/NPCs/Enemies/BP_EnemyCharacter.BP_EnemyCharacter_C"))
      (for _array_element _outactors
        (`GameplayStatics.ApplyDamage` _array_element (`self.Damage`) null self)))
    (:`then_1`
      (`|SpawnActorFromClass` "/Game/Blueprints/AnimatedSprites/BP_Explosion.BP_Explosion_C" (`KismetMathLibrary.MakeTransform` (`KismetMathLibrary.MakeVector` (- _returnvalue_x 100.0) _returnvalue_y _returnvalue_z)) "Undefined" "OverrideRootScale" null null))
    (:`then_2`
      (`self.K2_DestroyActor`))))

(fn `UserConstructionScript`
  (`parent.UserConstructionScript`))