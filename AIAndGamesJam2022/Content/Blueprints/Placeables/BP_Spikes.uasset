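; BP_Spikes is a placeable spike trap that deals continuous damage to enemies standing in its area.
; Sphere overlap events maintain a list of tracked BP_EnemyCharacter actors, with query collision switched on when the trap is placed.
; Each tick applies frame-time-scaled damage to every tracked enemy and drains the trap's own health by half that amount per enemy, calling OnPlaceableDestroyed when health runs out.
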(event `self.Sphere.OnComponentBeginOverlap`
  (params (OverlappedComponent :type "PrimitiveComponent Object Reference") (OtherActor :type "Actor Object Reference") (OtherComp :type "PrimitiveComponent Object Reference") (OtherBodyIndex :type Integer) (bFromSweep :type Boolean) (SweepResult :type "HitResult Structure (by ref)"))
  (bind _asbp_enemy_character (cast `/Game/NPCs/Enemies/BP_EnemyCharacter` OtherActor))
  (`KismetArrayLibrary.Array_Add` (`self.TrackedEnemies`) _asbp_enemy_character))

(event `self.Sphere.OnComponentEndOverlap`
  (params (OverlappedComponent :type "PrimitiveComponent Object Reference") (OtherActor :type "Actor Object Reference") (OtherComp :type "PrimitiveComponent Object Reference") (OtherBodyIndex :type Integer))
  (bind _asbp_enemy_character (cast `/Game/NPCs/Enemies/BP_EnemyCharacter` OtherActor))
  (`KismetArrayLibrary.Array_RemoveItem` (`self.TrackedEnemies`) _asbp_enemy_character))

(event `self.ReceiveTick`
  (params (DeltaSeconds :type "Float (single-precision)"))
  (bind _returnvalue (* DeltaSeconds (`self.Damage`)))
  (`parent.ReceiveTick` DeltaSeconds)
  (for _array_element (`self.TrackedEnemies`)
    (`GameplayStatics.ApplyDamage` _array_element _returnvalue null self)
    (bind _output_get (set `self.Health` (- (`self.Health`) (/ _returnvalue 2.0))))
    (if (<= _output_get 0.0)
      (`self.OnPlaceableDestroyed`))))

(fn `OnPlaced`
  (`parent.OnPlaced`)
  (`PrimitiveComponent.SetCollisionEnabled` (`self.Sphere`) "QueryOnly"))

(fn `UserConstructionScript`
  (`parent.UserConstructionScript`))