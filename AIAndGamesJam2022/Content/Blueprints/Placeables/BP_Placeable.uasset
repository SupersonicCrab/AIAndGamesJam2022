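; BP_Placeable is an actor placed on a build grid that can take damage and be destroyed.
; Placement makes its static mesh block a custom trace channel and applies the placed scale, while hide and unhide functions toggle mesh visibility.
; Damage lowers Health, and at zero or below the actor clears its reference on the Grid, unlocks it for building and destroys itself.
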(event `self.ReceiveAnyDamage`
  (params (Damage :type "Float (single-precision)") (DamageType :type "DamageType Object Reference") (InstigatedBy :type "Controller Object Reference") (DamageCauser :type "Actor Object Reference"))
  (bind _returnvalue (- (`self.Health`) Damage))
  (set `self.Health` _returnvalue)
  (if (<= _returnvalue 0.0)
    (`self.OnPlaceableDestroyed`)))

(fn `OnHidden`
  (`SceneComponent.SetHiddenInGame` (`self.StaticMesh`) true true))

(fn `OnPlaceableDestroyed`
  (`|ExecutionSequence`
    (:`then_0`
      (bind _grid (`self.Grid`)
        (:`then`
          (set `/Game/Blueprints/PlayArea/BP_Grid.Placeable` null _grid)
          (set `/Game/Blueprints/PlayArea/BP_Grid.bBuildLocked` false _grid))
        (:`else`)))
    (:`then_1`
      (`self.K2_DestroyActor`))))

(fn `OnPlaced`
  (`PrimitiveComponent.SetCollisionResponseToChannel` (`self.StaticMesh`) "ECC_GameTraceChannel2" "ECR_Block")
  (`SceneComponent.SetRelativeScale3D` (`self.StaticMesh`) (`self.PlacedScale`)))

(fn `OnUnhidden`
  (`SceneComponent.SetHiddenInGame` (`self.StaticMesh`) false true))

(fn `UserConstructionScript`)