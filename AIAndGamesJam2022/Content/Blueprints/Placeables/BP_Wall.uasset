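; BP_Wall is a placeable wall that plays metal sounds when damaged or destroyed.
; On placement it adds a nav modifier, makes its three meshes block a trace channel, unhides them and randomizes the yaw of the two extra meshes within ±ZDelta.
; Placement and destruction both request a check from the level's BP_ObstructionChecker.
; Damage, placement and destruction also run the parent class logic.
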(event `CheckForObstruction`
  (bind _returnvalue (`GameplayStatics.GetActorOfClass` "/Game/NPCs/BP_ObstructionChecker.BP_ObstructionChecker_C"))
  (`/Game/NPCs/BP_ObstructionChecker.RequestCheck` _returnvalue 1.0))

(event `self.ReceiveAnyDamage`
  (params (Damage :type "Float (single-precision)") (DamageType :type "DamageType Object Reference") (InstigatedBy :type "Controller Object Reference") (DamageCauser :type "Actor Object Reference"))
  (`GameplayStatics.PlaySoundAtLocation` "/Game/Assets/Audio/Effects/A_MetalHit.A_MetalHit" (`self.K2_GetActorLocation`) (struct) 1.0 1.0 0.0 null null null null)
  (`parent.ReceiveAnyDamage` Damage DamageType InstigatedBy DamageCauser))

(fn `OnPlaceableDestroyed`
  (`GameplayStatics.PlaySoundAtLocation` "/Game/Assets/Audio/Effects/A_MetalDestroyed.A_MetalDestroyed" (`self.K2_GetActorLocation`) (struct) 1.0 1.0 0.0 null null null null)
  (`self.CheckForObstruction`)
  (`parent.OnPlaceableDestroyed`))

(fn `OnPlaced`
  (`parent.OnPlaced`)
  (`AddComponent|NODE_AddNavModifierComponent-0`)
  (`PrimitiveComponent.SetCollisionResponseToChannel` (`self.StaticMesh`) "ECC_GameTraceChannel2" "ECR_Block")
  (`PrimitiveComponent.SetCollisionResponseToChannel` (`self.StaticMesh2`) "ECC_GameTraceChannel2" "ECR_Block")
  (`PrimitiveComponent.SetCollisionResponseToChannel` (`self.StaticMesh1`) "ECC_GameTraceChannel2" "ECR_Block")
  (`SceneComponent.SetHiddenInGame` (`self.StaticMesh`) false true)
  (`self.RandomizeExtraWalls`)
  (`self.CheckForObstruction`))

(fn `RandomizeExtraWalls`
  (bind _zdelta (`self.ZDelta`))
  (for _array_element (`|MakeArray` (`self.StaticMesh1`) (`self.StaticMesh2`))
    (bind (_relativerotation_roll _relativerotation_pitch) (`KismetMathLibrary.BreakRotator` (`SceneComponent.RelativeRotation` _array_element)))
    (`SceneComponent.K2_SetRelativeRotation` _array_element (`KismetMathLibrary.MakeRotator` _relativerotation_roll _relativerotation_pitch (`KismetMathLibrary.RandomFloatInRange` (* _zdelta -1.0) _zdelta)) false false)))

(fn `UserConstructionScript`
  (`parent.UserConstructionScript`))