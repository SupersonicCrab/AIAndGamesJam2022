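; Mouse-cursor player controller that directs an AI-controlled player character, operates weapons and handles workshop placement on grids.
; Interact release writes the interactable under the cursor to the AI's blackboard and confirms the hovered grid for the pending workshop; holding it fires a targeted weapon.
; While placing, Tick traces highlight unlocked grids and hide hovered placeables; Cancel clears placement.
; It also reports cursor aim location and whether it lies inside the play area.
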(event `InputAction|Cancel`
  (params (Key :type "Key Structure"))
  (:`Released`
    (set `self.PlaceableWorkshop` null)))

(event `InputAction|Interact`
  (params (Key :type "Key Structure"))
  (:`Pressed`
    (`self.FireWeapon` true))
  (:`Released`
    (`self.SetTargetInteractableCursor`)
    (`self.SelectGrid`)
    (`self.FireWeapon` false)))

(event `self.ReceiveBeginPlay`
  (`parent.ReceiveBeginPlay`)
  (set `self.bShowMouseCursor` true)
  (bind _returnvalue (`GameplayStatics.GetActorOfClass` "/Game/Blueprints/PlayArea/BP_PlayArea.BP_PlayArea_C"))
  (set `self.PlayArea` _returnvalue))

(event `self.ReceiveTick`
  (params (DeltaSeconds :type "Float (single-precision)"))
  (`parent.ReceiveTick` DeltaSeconds)
  (`self.UpdateHighlightedGrid`)
  (`self.UpdateHighlightedPlaceable`))

(fn `FireWeapon`
  (params (bFiring :type Boolean))
  (bind _targetinteractable (`self.TargetInteractable`)
    (:`then`
      (bind _asbp_weapon (cast `/Game/Blueprints/Interactables/Weapons/BP_Weapon` _targetinteractable))
      (set `/Game/Blueprints/Interactables/Weapons/BP_Weapon.bFiring` bFiring _asbp_weapon))
    (:`else`)))

(fn `GetCursorAimLocation`
  (returns (AimLocation :type "Vector Structure") (bWithinPlayArea :type Boolean))
  (bind _hitresult (`self.GetHitResultUnderCursorForObjects` (`|MakeArray` "ObjectTypeQuery1" :!type "EObjectTypeQuery Enum") true))
  (bind _collision (`/Game/Blueprints/PlayArea/BP_PlayArea.Collision` (`self.PlayArea`)))
  (return (`.Location` (`GameplayStatics.BreakHitResult` _hitresult)) (`KismetMathLibrary.IsPointInBoxWithTransform` (`.Location` (`GameplayStatics.BreakHitResult` _hitresult)) (`SceneComponent.K2_GetComponentToWorld` _collision) (`BoxComponent.GetScaledBoxExtent` _collision))))

(fn `HidePlaceable`
  (params (Placeable :type "/Game/Blueprints/Placeables/BP_Placeable Object Reference"))
  (bind _output_get (set `self.HighlightedPlaceable` Placeable))
  (`/Game/Blueprints/Placeables/BP_Placeable.OnHidden` _output_get))

(fn `HoverGrid`
  (params (HighlightedGrid :type "/Game/Blueprints/PlayArea/BP_Grid Object Reference"))
  (`/Game/Blueprints/PlayArea/BP_Grid.OnHoverStarted` HighlightedGrid)
  (set `self.HighlightedGrid` HighlightedGrid))

(fn `SelectGrid`
  (`self.UpdateHighlightedGrid`)
  (bind _highlightedgrid (`self.HighlightedGrid`)
    (:`then`
      (bind _placeableworkshop (`self.PlaceableWorkshop`)
        (:`then`
          (`/Game/Blueprints/Interactables/Workshops/PlaceableWorkshops/BP_PlaceableWorkshop.OnGridChosen` _placeableworkshop _highlightedgrid)
          (`self.UnHoverGrid`)
          (set `self.PlaceableWorkshop` null))
        (:`else`)))
    (:`else`)))

(fn `SetTargetInteractableCursor`
  (`self.PlayerBlackboard`
    (:`then`
      (bind _asbp_interactable (cast `/Game/Blueprints/Interactables/BP_Interactable` (`.HitActor` (`GameplayStatics.BreakHitResult` (`self.GetHitResultUnderCursorForObjects` (`|MakeArray` "ObjectTypeQuery7" :!type "EObjectTypeQuery Enum") false)))))
      (`BlackboardComponent.SetValueAsObject` (`self.PlayerBlackboard`) (`self.TargetInteractableName`) _asbp_interactable)
      (bind _targetinteractable (`self.TargetInteractable`)
        (:`then`
          (`/Game/Blueprints/Interactables/BP_Interactable.OnPlayerAIInteractionFinished` _targetinteractable self (`self.PlayerAIController`)))
        (:`else`
          _))
      (set `self.TargetInteractable` _asbp_interactable))
    (:`else`)))

(fn `SetupPlayer`
  (params (PlayerAIController :type "/Game/Blueprints/Player/BP_PlayerAIController Object Reference"))
  (bind _output_get (set `self.PlayerAIController` PlayerAIController))
  (set `self.PlayerBlackboard` (`AIBlueprintHelperLibrary.GetBlackboard` _output_get)))

(fn `UnhidePlaceable`
  (bind _highlightedplaceable (`self.HighlightedPlaceable`)
    (:`then`
      (`/Game/Blueprints/Placeables/BP_Placeable.OnUnhidden` _highlightedplaceable)
      (set `self.HighlightedPlaceable` null))
    (:`else`)))

(fn `UnHoverGrid`
  (bind _highlightedgrid (`self.HighlightedGrid`)
    (:`then`
      (`/Game/Blueprints/PlayArea/BP_Grid.OnHoverFinished` _highlightedgrid)
      (set `self.HighlightedGrid` null))
    (:`else`)))

(fn `UpdateHighlightedGrid`
  (`self.PlaceableWorkshop`
    (:`then`
      (bind _asbp_grid (cast `/Game/Blueprints/PlayArea/BP_Grid` (`.HitActor` (`GameplayStatics.BreakHitResult` (`self.GetHitResultUnderCursorForObjects` (`|MakeArray` "ObjectTypeQuery7" :!type "EObjectTypeQuery Enum") false))))
        (:`then`
          (if (not (`/Game/Blueprints/PlayArea/BP_Grid.bBuildLocked` _asbp_grid))
            (`|ExecutionSequence`
              (:`then_0`
                (`self.UnHoverGrid`))
              (:`then_1`
                (`self.HoverGrid` _asbp_grid)))))
        (:`CastFailed`
          (`self.UnHoverGrid`))))
    (:`else`
      (`self.UnHoverGrid`))))

(fn `UpdateHighlightedPlaceable`
  (`self.PlaceableWorkshop`
    (:`then`
      (bind _asbp_placeable (cast `/Game/Blueprints/Placeables/BP_Placeable` (`.HitActor` (`GameplayStatics.BreakHitResult` (`self.GetHitResultUnderCursorForObjects` (`|MakeArray` "ObjectTypeQuery8" :!type "EObjectTypeQuery Enum") false))))
        (:`then`
          (`|ExecutionSequence`
            (:`then_0`
              (`self.UnhidePlaceable`))
            (:`then_1`
              (`self.HidePlaceable` _asbp_placeable))))
        (:`CastFailed`
          (`self.UnhidePlaceable`))))
    (:`else`
      (`self.UnhidePlaceable`))))

(fn `UserConstructionScript`)