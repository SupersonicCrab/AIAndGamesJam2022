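; BP_Gate is a destructible gate that opens for allowed classes when no enemies are nearby and closes only once no allowed characters remain.
; A sphere trigger tracks allowed and enemy characters, driving the door Timeline and sounds.
; It writes bAtGate to NPC blackboards and bEnemiesNearDoor to the robot's blackboard.
; Damage plays a hit effect and passes to GM_DwarfStuck, whose result decides whether the gate is destroyed.
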(event `self.Sphere.OnComponentBeginOverlap`
  (params (OverlappedComponent :type "PrimitiveComponent Object Reference") (OtherActor :type "Actor Object Reference") (OtherComp :type "PrimitiveComponent Object Reference") (OtherBodyIndex :type Integer) (bFromSweep :type Boolean) (SweepResult :type "HitResult Structure (by ref)"))
  (`self.SetAtGate` OtherActor true)
  (if (`KismetArrayLibrary.Array_Contains` (`self.ClassToAllow`) (`GameplayStatics.GetObjectClass` OtherActor))
    (`KismetArrayLibrary.Array_Add` (`self.AllowedCharacters`) OtherActor)
    (`self.Open`)
    (`self.UpdateRobotBlackboard`)
    (else
      (cast `/Game/NPCs/Enemies/BP_EnemyCharacter` OtherActor)
      (`KismetArrayLibrary.Array_Add` (`self.EnemyCharacters`) OtherActor)
      (`self.Close`)
      (`self.UpdateRobotBlackboard`))))

(event `self.Sphere.OnComponentEndOverlap`
  (params (OverlappedComponent :type "PrimitiveComponent Object Reference") (OtherActor :type "Actor Object Reference") (OtherComp :type "PrimitiveComponent Object Reference") (OtherBodyIndex :type Integer))
  (`self.SetAtGate` OtherActor)
  (`KismetArrayLibrary.Array_RemoveItem` (`self.AllowedCharacters`) OtherActor)
  (`KismetArrayLibrary.Array_RemoveItem` (`self.EnemyCharacters`) OtherActor)
  (if (or (`KismetArrayLibrary.Array_IsEmpty` (`self.AllowedCharacters`)) (not (`KismetArrayLibrary.Array_IsEmpty` (`self.EnemyCharacters`))))
    (`self.Close`)
    (`self.UpdateRobotBlackboard`)))

(event `self.ReceiveBeginPlay`
  (`parent.ReceiveBeginPlay`)
  (bind _asgm_dwarf_stuck (cast `/Game/Blueprints/GM_DwarfStuck` (`GameplayStatics.GetGameMode`)))
  (set `self.GameMode` _asgm_dwarf_stuck))

(fn `Close`
  (if (and (`KismetArrayLibrary.Array_IsEmpty` (`self.AllowedCharacters`)) (not (`self.bClosed`)))
    (`TimelineComponent.ReverseFromEnd` (`self.OpenAnimation`))
    (set `self.bClosed` true)
    (`GameplayStatics.PlaySoundAtLocation` "/Game/Assets/Audio/Effects/A_DoorClose.A_DoorClose" (`self.K2_GetActorLocation`) (struct) 1.0 1.0 0.0 null null null null)))

(fn `Open`
  (if (`self.bClosed`)
    (if (`KismetArrayLibrary.Array_IsEmpty` (`self.EnemyCharacters`))
      (set `self.bClosed` false)
      (`TimelineComponent.PlayFromStart` (`self.OpenAnimation`))
      (`GameplayStatics.PlaySoundAtLocation` "/Game/Assets/Audio/Effects/A_DoorOpen.A_DoorOpen" (`self.K2_GetActorLocation`) (struct) 1.0 1.0 0.0 null null null null))))

(fn `ReceiveAnyDamage`
  (params (Damage :type "Float (single-precision)") (DamageType :type "DamageType Object Reference") (InstigatedBy :type "Controller Object Reference") (DamageCauser :type "Actor Object Reference"))
  (bind _hurtanimation (`self.HurtAnimation`))
  (`|ExecutionSequence`
    (:`then_0`
      (`GameplayStatics.PlaySoundAtLocation` "/Game/Assets/Audio/Effects/A_MetalHit.A_MetalHit" (`self.K2_GetActorLocation`) (struct) 1.0 1.0 0.0 null null null null)
      (if (not (`TimelineComponent.IsPlaying` _hurtanimation))
        (`TimelineComponent.PlayFromStart` _hurtanimation)))
    (:`then_1`
      (bind _blost (`/Game/Blueprints/GM_DwarfStuck.DealDamage` (`self.GameMode`) Damage))
      (if _blost
        (`GameplayStatics.PlaySoundAtLocation` "/Game/Assets/Audio/Effects/A_MetalDestroyed.A_MetalDestroyed" (`self.K2_GetActorLocation`) (struct) 1.0 1.0 0.0 null null null null)
        (`self.K2_DestroyActor`)))))

(fn `SetAtGate`
  (params (NPC :type "Actor Object Reference") (bAtGate :type Boolean))
  (bind _asbp_npccharacter (cast `/Game/NPCs/BP_NPCCharacter` NPC))
  (if (not (`self.IsActorBeingDestroyed` _asbp_npccharacter))
    (bind _blackboard (`/Game/NPCs/BP_NPCCharacter.Blackboard` _asbp_npccharacter)
      (:`then`
        (`BlackboardComponent.SetValueAsBool` _blackboard "bAtGate" bAtGate))
      (:`else`))))

(fn `TestDamage`
  (`GameplayStatics.ApplyDamage` self 100.0))

(fn `UpdateRobotBlackboard`
  (bind _robotblackboard (`self.RobotBlackboard`))
  (bind _returnvalue (`KismetArrayLibrary.Array_IsNotEmpty` (`self.EnemyCharacters`)))
  (if (!= _returnvalue (`BlackboardComponent.GetValueAsBool` _robotblackboard "bEnemiesNearDoor"))
    (`BlackboardComponent.SetValueAsBool` _robotblackboard "bEnemiesNearDoor" _returnvalue)))

(fn `UserConstructionScript`)