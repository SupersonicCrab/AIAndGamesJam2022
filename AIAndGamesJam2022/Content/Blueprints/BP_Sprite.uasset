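; BP_Sprite is a Paper2D sprite actor with a FaceCamera function meant to orient its sprite toward the player camera.
; The construction script calls FaceCamera, with no per-frame update in the graphs shown.
; It keeps the sprite's pitch, sets yaw from Offset, and adds Offset roll to the look-at roll.
; Since FindLookAtRotation yields zero roll, camera position does not actually affect the result.
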(fn `FaceCamera`
  (locals (Offset :type "Rotator Structure" :default (struct :`Yaw` 90.0 :`Roll` -40.0)))
  (bind (_offset_roll _offset_pitch _offset_yaw) (`KismetMathLibrary.BreakRotator` (`local.Offset`)))
  (bind (_returnvalue_roll _returnvalue_pitch) (`KismetMathLibrary.BreakRotator` (`SceneComponent.K2_GetComponentRotation` (`self.PaperSprite`))))
  (bind _returnvalue_roll_2 (`KismetMathLibrary.BreakRotator` (`KismetMathLibrary.FindLookAtRotation` (`self.K2_GetActorLocation`) (`PlayerCameraManager.GetCameraLocation` (`GameplayStatics.GetPlayerCameraManager` 0)))))
  (`SceneComponent.K2_SetWorldRotation` (`self.PaperSprite`) (`KismetMathLibrary.MakeRotator` (+ _returnvalue_roll_2 _offset_roll) _returnvalue_pitch _offset_yaw) false false))

(fn `UserConstructionScript`
  (`self.FaceCamera`))